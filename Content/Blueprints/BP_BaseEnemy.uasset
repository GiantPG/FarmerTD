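; BP_BaseEnemy is a base enemy actor that travels along a given spline path and is destroyed when damage depletes its health.
; Init stores the spline and sets the Move timeline's play rate from spline length and Speed, so travel speed is independent of path length.
; Each timeline update moves it to the interpolated spline distance, keeping its own Z and facing along the tangent.
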(event Custom|Init
  (params (SplineToFollow :type Spline%20Component%20Object%20Reference))
  ;[1 1 1 1 36] Init
  (Variables|Default|SetSplineToFollow SplineToFollow)
  (Components|Timeline|SetPlayRate (Variables|Default|GetMove) (/ 1.0 (/ (Spline|GetSplineLength (Variables|Default|GetSplineToFollow)) (Variables|Default|GetSpeed))))
  (CallFunction|MoveAlongSpline))

(event Custom|MoveAlongSpline
  (bind _splinetofollow (Variables|Default|GetSplineToFollow))
  (bind _splinetofollow_2 (Variables|Default|GetSplineToFollow))
  ;[1 1 1 1 36] Movement
  (bind _alpha (Timeline|Move PlayFromStart)
    (:Update
      (Utilities|IsValid _splinetofollow_2
        (:Is%20Valid
          (Transformation|SetActorLocationAndRotation (Math|Vector|MakeVector (.x (Spline|GetLocationatDistanceAlongSpline _splinetofollow_2 (Math|Float|Lerp 0.0 (Spline|GetDistanceAlongSplineatSplinePoint _splinetofollow (- (Spline|GetNumberOfSplinePoints _splinetofollow) 1)) _alpha) "World")) (.y (Spline|GetLocationatDistanceAlongSpline _splinetofollow_2 (Math|Float|Lerp 0.0 (Spline|GetDistanceAlongSplineatSplinePoint _splinetofollow (- (Spline|GetNumberOfSplinePoints _splinetofollow) 1)) _alpha) "World")) (.z (Transformation|GetActorLocation))) (Math|Conversions|RotationFromXVector (Spline|GetTangentatDistanceAlongSpline (Variables|Default|GetSplineToFollow) (Math|Float|Lerp 0.0 (Spline|GetDistanceAlongSplineatSplinePoint _splinetofollow (- (Spline|GetNumberOfSplinePoints _splinetofollow) 1)) _alpha) "World"))))))))

(event Game|Damage|EventAnyDamage
  (params (Damage :type Float%20%28single-precision%29) (DamageType :type Damage%20Type%20Object%20Reference) (InstigatedBy :type Controller%20Object%20Reference) (DamageCauser :type Actor%20Object%20Reference))
  ;[1 1 1 1 36] Damage
  (bind _output_get (Variables|Default|SetCurrentHealth (- (Variables|Default|GetCurrentHealth) Damage)))
  (if (<= _output_get 0.0)
    (Actor|DestroyActor)))

(fn ConstructionScript)