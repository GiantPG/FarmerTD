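; BP_Well is a well actor that refills Farmer Ted's watering can.
; Box overlap toggles input, the prompt widget and a Gate, so Interact only works while the farmer is nearby.
; Interact starts a looping timer, apparently driving RefillCan, which passes RefillSpeed to the cached character's TransferWaterMessage.
; Leaving the box clears the timer; an older direct clamp-and-stop refill is left unconnected.
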(event OnComponentBeginOverlap(Box)
  (params (OverlappedComponent :type Primitive%20Component%20Object%20Reference) (OtherActor :type Actor%20Object%20Reference) (OtherComp :type Primitive%20Component%20Object%20Reference) (OtherBodyIndex :type Integer) (bFromSweep :type Boolean) (SweepResult :type Hit%20Result%20Structure%20%28by%20ref%29))
  (Utilities|Casting|CastToBP_FarmerTed_SpriteMinimap OtherActor)
  (Input|EnableInput (Game|GetPlayerController 0))
  (Development|SetHiddeninGame (Variables|Default|GetWidget) false false)
  (Variables|Default|SetNear%20Well true)
  (Utilities|FlowControl|Gate true) ; enters at Open
)

(event OnComponentEndOverlap(Box)
  (params (OverlappedComponent :type Primitive%20Component%20Object%20Reference) (OtherActor :type Actor%20Object%20Reference) (OtherComp :type Primitive%20Component%20Object%20Reference) (OtherBodyIndex :type Integer))
  (Utilities|FlowControl|Sequence
    (:then_0
      (Utilities|Casting|CastToBP_FarmerTed_SpriteMinimap OtherActor)
      (Input|DisableInput (Game|GetPlayerController 0))
      (Development|SetHiddeninGame (Variables|Default|GetWidget) true false)
      (Variables|Default|SetNear%20Well false)
      (Utilities|FlowControl|Gate true) ; enters at Close
    )
    (:then_1
      (Utilities|Time|ClearandInvalidateTimerbyHandle (Variables|Default|GetClear%20Timer)))))

(event Custom|RefillCan
  (Class|BPIWaterTransferable|TransferWater(Message) (Variables|Default|GetAs%20BP%20Farmer%20Ted%20Sprite%20Minimap) (Variables|Default|GetRefillSpeed)))

(event EventBeginPlay
  (bind _asbp_farmer_ted_sprite_minimap (Utilities|Casting|CastToBP_FarmerTed_SpriteMinimap (Game|GetPlayerCharacter 0)))
  (Variables|Default|SetAs%20BP%20Farmer%20Ted%20Sprite%20Minimap _asbp_farmer_ted_sprite_minimap))

(event Collision|EventActorBeginOverlap
  (params (OtherActor :type Actor%20Object%20Reference)))

(event EventTick
  (params (DeltaSeconds :type Float%20%28single-precision%29)))

(event Input|ActionEvents|InputActionInteract
  (params (Key :type Key%20Structure))
  (:Pressed
    (Utilities|FlowControl|Gate true
      (:Exit
        (if (Variables|Default|GetNear%20Well)
          (bind _returnvalue (Utilities|Time|SetTimerbyEvent (EventDispatchers|CreateEvent :!event Custom|RefillCan) 0.1 true))
          (Variables|Default|SetClear%20Timer _returnvalue))))))

(fn ConstructionScript)