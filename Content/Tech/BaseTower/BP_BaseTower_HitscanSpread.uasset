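; Tower-defense turret that shoots enemies with randomly spread hitscan traces and has a draining Hydration value that destroys it at zero.
; Each tick it picks a BP_BaseEnemy in range with line of sight, rotates TowerTop toward it and fires once aligned and off cooldown.
; Fire uses a delayed DoN loop for multi-shot bursts, damaging whatever each trace hits.
; UpgradeLVL1 rescales damage, rotation speed, fire rate and range.
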(event Custom|Fire
  (bind _maxspread (Variables|Default|GetMaxSpread))
  (bind _target (Variables|Private|GetTarget))
  (bind _minspread (Variables|Default|GetMinSpread))
  (bind _returnvalue (Transformation|GetActorLocation _target))
  (Variables|Private|SetLast%20Time%20Tower%20Fired (Utilities|Time|GetGameTimeinSeconds))
  (Utilities|FlowControl|Sequence
    (:then_0
      (goto _label Reset))
    (:then_1
      (Utilities|FlowControl|DoN (Variables|Default|GetFireHowManyAtOnce) :!label _label ; An optional how many times to fire in one cycle, very useful for a two barrel minigun
        (:Exit
          (Utilities|IsValid (Variables|Private|GetTarget)
            (:Is%20Valid
              (bind _outhit (Collision|LineTraceByChannel (.location (Transformation|GetWorldTransform (Variables|Default|GetArrow))) (Math|Vector|MakeVector (+ (.x _returnvalue) (Math|Random|RandomFloatinRange _minspread _maxspread)) (+ (.y _returnvalue) (Math|Random|RandomFloatinRange _minspread _maxspread)) (+ (.z _returnvalue) (Math|Random|RandomFloatinRange _minspread _maxspread))) "TraceTypeQuery1" false 0 "Persistent"))
              (Development|PrintString "Hit")
              (Game|Damage|ApplyDamage (.hitactor _outhit) (Variables|Upgrades|GetS%20Damage) 0 0)
              (Utilities|FlowControl|Delay 0.1)
              (goto _label))))))))

(event Custom|HydrationEvent
  ;[1 1 1] Drain Hydration
  (bind _output_get (Variables|Default|SetHydration (Math|Integer|Clamp(Integer) (- (Variables|Default|GetHydration) 1) 0 100)))
  (if (== _output_get 0)
    (Actor|DestroyActor)
    (else
      (Development|PrintString (Utilities|String|ToString(Integer) (Variables|Default|GetHydration)))
      (Utilities|FlowControl|Delay 5.0)
      (CallFunction|HydrationEvent))))

(event Custom|Upgrade%20LVL1
  (params (Tower%20Damage :type Float%20%28double-precision%29) (Rotation%20Speed :type Float%20%28double-precision%29) (Fire%20Rate :type Float%20%28double-precision%29) (Tower%20Range :type Float%20%28double-precision%29))
  (Variables|Upgrades|SetS%20Damage (* Tower%20Damage 1.2))
  (Variables|Upgrades|SetS%20Rotation%20Speed (* Rotation%20Speed 1.2))
  (Variables|Upgrades|SetS%20Fire%20Rate (* Fire%20Rate -1.2))
  (Variables|Upgrades|SetS%20Tower%20Range (* Tower%20Range 1.2)))

(event EventBeginPlay
  (Variables|Upgrades|SetS%20Damage 5.0)
  (Variables|Upgrades|SetS%20Tower%20Range 5e+02)
  (Variables|Upgrades|SetS%20Fire%20Rate 1.0)
  (Class|BPIWaterable|Water(Message) self 0.0)
  (Utilities|Time|SetTimerbyEvent (EventDispatchers|CreateEvent :!event Custom|HydrationEvent) 1.0))

(event EventTick
  (params (DeltaSeconds :type Float%20%28single-precision%29))
  (CallFunction|FindTarget)
  (Variables|Private|GetTarget
    (:then
      (CallFunction|RotateTowerTop DeltaSeconds)
      (CallFunction|UpdateFire))
    (:else)))

(fn ConstructionScript)

(fn FindTarget
  (LocalVariables|SetBestDistance (+ (Variables|Upgrades|GetS%20Tower%20Range) 1.0))
  (bind _outactors (Collision|SphereOverlapActors (Transformation|GetActorLocation) (Variables|Upgrades|GetS%20Tower%20Range) (Utilities|Array|MakeArray "ObjectTypeQuery3") "/Game/Blueprints/BP_BaseEnemy.BP_BaseEnemy_C"))
  (for _array_element _outactors
    (bind _output_get (LocalVariables|SetCurrentTarget _array_element))
    (if (<= (Math|Vector|Distance(Vector) (Transformation|GetActorLocation _output_get) (Transformation|GetActorLocation)) (LocalVariables|GetBestDistance)) ; Closest Target
      (bind _result (CallFunction|SightOfTarget (Transformation|GetWorldLocation (Variables|Default|GetTowerTop)) (Transformation|GetActorLocation (LocalVariables|GetCurrentTarget)) (Utilities|Array|MakeArray self (LocalVariables|GetCurrentTarget))))
      (if _result
        (LocalVariables|SetBestTarget (LocalVariables|GetCurrentTarget))
        (LocalVariables|SetBestDistance (LocalVariables|GetCurrentDistance)))))
  (Variables|Private|SetTarget (LocalVariables|GetBestTarget)))

(fn RotateTowerTop
  (params (Delta%20Seconds :type Float%20%28double-precision%29))
  (Transformation|SetWorldRotation (Variables|Default|GetTowerTop) (Class|KismetMathLibrary|RInterptoConstant (Transformation|GetWorldRotation (Variables|Default|GetTowerTop)) (Math|Rotator|FindLookatRotation (Transformation|GetWorldLocation (Variables|Default|GetTowerTop)) (Transformation|GetActorLocation (Variables|Private|GetTarget))) Delta%20Seconds (Variables|Upgrades|GetS%20Rotation%20Speed)) false false))

(fn UpdateFire
  ;[1 1 1] Cooldown for Firing
  (if (> (- (Utilities|Time|GetGameTimeinSeconds) (Variables|Private|GetLast%20Time%20Tower%20Fired)) (Variables|Upgrades|GetS%20Fire%20Rate))
    (if (> (Math|Vector|DotProduct (Math|Vector|GetUnitDirection(Vector) (Transformation|GetWorldLocation (Variables|Default|GetTowerTop)) (Transformation|GetActorLocation (Variables|Private|GetTarget))) (Math|Vector|GetForwardVector (Variables|Default|GetTowerTop))) 0.99999) ; Turret Facing Target
      (CallFunction|Fire))))