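; Chili Tower, a tower subclass that fires bursts of chilli projectiles at its target.
; BeginPlay sets the display name and runs the parent setup.
; Fire records the shot time, resets a DoN counter and enters it, spawning a projectile at the Arrow's transform.
; A short Delay re-enters the DoN, looping up to FireHowManyAtOnce shots while the Target stays valid.
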(event EventBeginPlay
  (Variables|Default|SetName "Chili Tower")
  (|CallParentFunction))

(event Collision|EventActorBeginOverlap
  (params (OtherActor :type Actor%20Object%20Reference)))

(event EventTick
  (params (DeltaSeconds :type Float%20%28single-precision%29)))

(event EventFire
  (bind _arrow (Variables|Default|GetArrow))
  (bind _returnvalue (Transformation|GetWorldTransform _arrow))
  (Variables|Default|SetLast%20Time%20Tower%20Fired (Utilities|Time|GetGameTimeinSeconds))
  (Utilities|FlowControl|Sequence
    (:then_0
      (goto _label Reset))
    (:then_1
      (Utilities|FlowControl|DoN (Variables|Default|GetFireHowManyAtOnce) :!label _label
        (:Exit
          (Utilities|IsValid (Variables|Default|GetTarget)
            (:Is%20Valid
              (Game|SpawnActorfromClass "/Game/Tech/BaseProjectile/BP_Projectile_Chilli.BP_Projectile_Chilli_C" (Math|Transform|MakeTransform (.location _returnvalue) (.rotation _returnvalue) "1.000000,1.000000,1.000000") "Undefined" 0 0)
              (Utilities|FlowControl|Delay 0.1)
              (goto _label))))))))

(fn ConstructionScript
  (|CallParentFunction))