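; Base tower Blueprint that targets enemies and withers when its hydration runs out, until watered.
; A range sphere tracks overlapping BP_BaseEnemy actors for random target selection, and watering rescans it.
; Gated Delay loops turn the yaw pivot and pitch head toward the target, or back to neutral without one.
; Line of sight, cooldown and a dot-product alignment check gate an empty Fire event; three upgrade events scale the stats.
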(event OnComponentBeginOverlap(Sphere)
  (params (OverlappedComponent :type Primitive%20Component%20Object%20Reference) (OtherActor :type Actor%20Object%20Reference) (OtherComp :type Primitive%20Component%20Object%20Reference) (OtherBodyIndex :type Integer) (bFromSweep :type Boolean) (SweepResult :type Hit%20Result%20Structure%20%28by%20ref%29))
  ;[1 1 1] Detect all enemies which have overlapped
  (if (not (Variables|Default|GetWithered))
    (bind _asbp_base_enemy (Utilities|Casting|CastToBP_BaseEnemy OtherActor))
    (Utilities|Array|Add (Variables|TargetDetection|GetEnemiesInRange) _asbp_base_enemy)
    (Utilities|IsValid (Variables|TargetDetection|GetTarget)
      (:Is%20Not%20Valid
        (CallFunction|SelectTarget)))))

(event OnComponentEndOverlap(Sphere)
  (params (OverlappedComponent :type Primitive%20Component%20Object%20Reference) (OtherActor :type Actor%20Object%20Reference) (OtherComp :type Primitive%20Component%20Object%20Reference) (OtherBodyIndex :type Integer))
  (bind _enemiesinrange (Variables|TargetDetection|GetEnemiesInRange))
  ;[1 1 1] Detect all enemies which have overlapped
  (if (not (Variables|Default|GetWithered))
    (bind _asbp_base_enemy (Utilities|Casting|CastToBP_BaseEnemy OtherActor))
    (if (Utilities|Array|ContainsItem _enemiesinrange _asbp_base_enemy)
      (Utilities|Array|RemoveItem _enemiesinrange _asbp_base_enemy)
      (if (== _asbp_base_enemy (Variables|TargetDetection|GetTarget))
        (Variables|TargetDetection|SetTarget 0)
        (CallFunction|SelectTarget)))))

(event Custom|Upgrade%20LVL1
  (Variables|Upgrade|SetS%20Damage (* (Variables|Upgrade|GetS%20Damage) 1.3))
  (Variables|Upgrade|SetS%20Rotation%20Speed (* (Variables|Upgrade|GetS%20Rotation%20Speed) 1.2))
  (Variables|Upgrade|SetS%20Fire%20Rate (* (Variables|Upgrade|GetS%20Fire%20Rate) -0.5))
  (Variables|Upgrade|SetS%20Tower%20Range (* (Variables|Upgrade|GetS%20Tower%20Range) 1.2)))

(event Custom|ContinueReset
  (bind _returnvalue (Utilities|Time|GetWorldDeltaSeconds))
  (bind _towertopcentre (Variables|Default|GetTowerTopCentre))
  (bind _towertop (Variables|Default|GetTowerTop))
  (bind _relativerotation (Variables|/Script/Engine.SceneComponent|GetRelativeRotation _towertop))
  (bind _relativerotation_2 (Variables|/Script/Engine.SceneComponent|GetRelativeRotation _towertopcentre))
  (bind _returnvalue_2 (Class|KismetMathLibrary|RInterptoConstant _relativerotation "0, 0, 0" _returnvalue 0.0))
  (bind _returnvalue_3 (Class|KismetMathLibrary|RInterptoConstant _relativerotation_2 "0, 0, 0" _returnvalue 0.0))
  ;[1 1 1] Reset Rotation
  (Utilities|FlowControl|Gate true
    (:Exit
      (Utilities|IsValid (Variables|TargetDetection|GetTarget)
        (:Is%20Valid
          (CallFunction|CancelReset :!label _label))
        (:Is%20Not%20Valid
          (if (and (Utilities|Operators|EqualEqual :A _returnvalue_3 :ErrorTolerance 0.0001) (Utilities|Operators|EqualEqual :A _returnvalue_2 :ErrorTolerance 0.0001))
            (goto _label)
            (else
              (Transformation|SetRelativeRotation (Variables|Default|GetTowerTopCentre) _returnvalue_3 false false)
              (Transformation|SetRelativeRotation (Variables|Default|GetTowerTop) _returnvalue_2 false false)
              (Utilities|FlowControl|Delay (Utilities|Time|GetWorldDeltaSeconds))
              (CallFunction|ContinueReset))))))))

(event Custom|CancelReset
  (bind _returnvalue (Utilities|Time|GetWorldDeltaSeconds))
  (bind _towertopcentre (Variables|Default|GetTowerTopCentre))
  (bind _towertop (Variables|Default|GetTowerTop))
  (bind _relativerotation (Variables|/Script/Engine.SceneComponent|GetRelativeRotation _towertop))
  (bind _relativerotation_2 (Variables|/Script/Engine.SceneComponent|GetRelativeRotation _towertopcentre))
  (bind _returnvalue_2 (Class|KismetMathLibrary|RInterptoConstant _relativerotation "0, 0, 0" _returnvalue 0.0))
  (bind _returnvalue_3 (Class|KismetMathLibrary|RInterptoConstant _relativerotation_2 "0, 0, 0" _returnvalue 0.0))
  ;[1 1 1] Reset Rotation
  (Utilities|FlowControl|Gate true) ; enters at Close
)

(event Custom|Fire)

(event Custom|Stop
  (Utilities|FlowControl|Delay (Utilities|Time|GetWorldDeltaSeconds))
  (CallFunction|ContinueAim))

(event Custom|HydrationEvent
  ;[1 1 1] Drain Hydration
  (bind _output_get (Variables|Default|SetHydration (Math|Integer|Clamp(Integer) (- (Variables|Default|GetHydration) 1) 0 100)))
  (if (<= _output_get 0)
    (Variables|Default|SetWithered true))
  (Rendering|Components|TextRender|SetText (Variables|Default|GetTextRender) (Utilities|Text|ToText(Integer) (Variables|Default|GetHydration))))

(event Custom|StartAiming
  (bind _returnvalue (Utilities|Time|GetWorldDeltaSeconds))
  (bind _s_rotation_speed (Variables|Upgrade|GetS%20Rotation%20Speed))
  ;[1 1 1] Look At Target
  (Utilities|FlowControl|Sequence
    (:then_0
      (goto _label Open))
    (:then_1
      (Utilities|FlowControl|Gate true :!label _label
        (:Exit
          (Utilities|IsValid (Variables|TargetDetection|GetTarget)
            (:Is%20Valid
              (Variables|TargetDetection|SetTargetLocation (Transformation|GetActorLocation (Variables|TargetDetection|GetTarget)))
              (Transformation|SetRelativeRotation (Variables|Default|GetTowerTopCentre) (Class|KismetMathLibrary|RInterptoConstant (Variables|/Script/Engine.SceneComponent|GetRelativeRotation (Variables|Default|GetTowerTopCentre)) (Math|Rotator|MakeRotator 0.0 0.0 (.Yaw (Math|Rotator|BreakRotator (Math|Rotator|MakeRotfromX (Math|Transform|InverseTransformDirection (Transformation|GetActorTransform) (- (Variables|TargetDetection|GetTargetLocation) (Transformation|GetWorldLocation (Variables|Default|GetTowerTop)))))))) _returnvalue _s_rotation_speed) false false)
              (Transformation|SetRelativeRotation (Variables|Default|GetTowerTop) (Class|KismetMathLibrary|RInterptoConstant (Variables|/Script/Engine.SceneComponent|GetRelativeRotation (Variables|Default|GetTowerTop)) (Math|Rotator|MakeRotator 0.0 (.Pitch (Math|Rotator|BreakRotator (Math|Rotator|MakeRotfromX (Math|Transform|InverseTransformDirection (Transformation|GetActorTransform) (- (Variables|TargetDetection|GetTargetLocation) (Transformation|GetWorldLocation (Variables|Default|GetTowerTop))))))) 0.0) _returnvalue _s_rotation_speed) false false)
              (Utilities|IsValid (Variables|TargetDetection|GetTarget)
                (:Is%20Valid
                  (bind _result (CallFunction|SightOfTarget (Transformation|GetWorldLocation (Variables|Default|GetArrow)) (Transformation|GetActorLocation (Variables|TargetDetection|GetTarget)) (Utilities|Array|MakeArray self (Variables|TargetDetection|GetTarget))))
                  (if _result
                    (CallFunction|UpdateFire)
                    (else
                      (CallFunction|Stop)))
                  (Utilities|FlowControl|Delay (Utilities|Time|GetWorldDeltaSeconds))
                  (CallFunction|ContinueAim))))
            (:Is%20Not%20Valid
              (CallFunction|CancelAim)
              (CallFunction|StartReset))))))))

(event Custom|Upgrade%20LVL3
  (Variables|Upgrade|SetS%20Damage (* (Variables|Upgrade|GetS%20Damage) 1.3))
  (Variables|Upgrade|SetS%20Rotation%20Speed (* (Variables|Upgrade|GetS%20Rotation%20Speed) 1.2))
  (Variables|Upgrade|SetS%20Fire%20Rate (* (Variables|Upgrade|GetS%20Fire%20Rate) -0.5))
  (Variables|Upgrade|SetS%20Tower%20Range (* (Variables|Upgrade|GetS%20Tower%20Range) 1.2)))

(event Custom|Upgrade%20LVL2
  (Variables|Upgrade|SetS%20Damage (* (Variables|Upgrade|GetS%20Damage) 1.3))
  (Variables|Upgrade|SetS%20Rotation%20Speed (* (Variables|Upgrade|GetS%20Rotation%20Speed) 1.2))
  (Variables|Upgrade|SetS%20Fire%20Rate (* (Variables|Upgrade|GetS%20Fire%20Rate) -0.5))
  (Variables|Upgrade|SetS%20Tower%20Range (* (Variables|Upgrade|GetS%20Tower%20Range) 1.2)))

(event Custom|StartReset
  (bind _returnvalue (Utilities|Time|GetWorldDeltaSeconds))
  (bind _towertopcentre (Variables|Default|GetTowerTopCentre))
  (bind _towertop (Variables|Default|GetTowerTop))
  (bind _relativerotation (Variables|/Script/Engine.SceneComponent|GetRelativeRotation _towertop))
  (bind _relativerotation_2 (Variables|/Script/Engine.SceneComponent|GetRelativeRotation _towertopcentre))
  (bind _returnvalue_2 (Class|KismetMathLibrary|RInterptoConstant _relativerotation "0, 0, 0" _returnvalue 0.0))
  (bind _returnvalue_3 (Class|KismetMathLibrary|RInterptoConstant _relativerotation_2 "0, 0, 0" _returnvalue 0.0))
  ;[1 1 1] Reset Rotation
  (Utilities|FlowControl|Sequence
    (:then_0
      (goto _label Open))
    (:then_1
      (Utilities|FlowControl|Gate true :!label _label
        (:Exit
          (Utilities|IsValid (Variables|TargetDetection|GetTarget)
            (:Is%20Valid
              (CallFunction|CancelReset :!label _label_2))
            (:Is%20Not%20Valid
              (if (and (Utilities|Operators|EqualEqual :A _returnvalue_3 :ErrorTolerance 0.0001) (Utilities|Operators|EqualEqual :A _returnvalue_2 :ErrorTolerance 0.0001))
                (goto _label_2)
                (else
                  (Transformation|SetRelativeRotation (Variables|Default|GetTowerTopCentre) _returnvalue_3 false false)
                  (Transformation|SetRelativeRotation (Variables|Default|GetTowerTop) _returnvalue_2 false false)
                  (Utilities|FlowControl|Delay (Utilities|Time|GetWorldDeltaSeconds))
                  (CallFunction|ContinueReset))))))))))

(event Custom|SelectTarget
  (bind _enemiesinrange (Variables|TargetDetection|GetEnemiesInRange))
  ;[1 1 1] Select Enemy
  (if (Utilities|Array|IsValidIndex _enemiesinrange)
    (Variables|TargetDetection|SetTarget (Utilities|Array|Get(acopy) _enemiesinrange (Math|Random|RandomIntegerinRange 0 (Utilities|Array|LastIndex _enemiesinrange))))
    (CallFunction|StartAiming)
    (else
      (CallFunction|StartReset))))

(event Custom|CancelAim
  (bind _returnvalue (Utilities|Time|GetWorldDeltaSeconds))
  (bind _s_rotation_speed (Variables|Upgrade|GetS%20Rotation%20Speed))
  ;[1 1 1] Look At Target
  (Utilities|FlowControl|Gate true) ; enters at Close
)

(event Custom|ContinueAim
  (bind _returnvalue (Utilities|Time|GetWorldDeltaSeconds))
  (bind _s_rotation_speed (Variables|Upgrade|GetS%20Rotation%20Speed))
  (bind _withered (Variables|Default|GetWithered))
  ;[1 1 1] Look At Target
  (Utilities|IsValid (Variables|TargetDetection|GetTarget)
    (:Is%20Valid
      (if (not _withered)
        (Utilities|FlowControl|Gate true
          (:Exit
            (Utilities|IsValid (Variables|TargetDetection|GetTarget)
              (:Is%20Valid
                (Variables|TargetDetection|SetTargetLocation (Transformation|GetActorLocation (Variables|TargetDetection|GetTarget)))
                (Transformation|SetRelativeRotation (Variables|Default|GetTowerTopCentre) (Class|KismetMathLibrary|RInterptoConstant (Variables|/Script/Engine.SceneComponent|GetRelativeRotation (Variables|Default|GetTowerTopCentre)) (Math|Rotator|MakeRotator 0.0 0.0 (.Yaw (Math|Rotator|BreakRotator (Math|Rotator|MakeRotfromX (Math|Transform|InverseTransformDirection (Transformation|GetActorTransform) (- (Variables|TargetDetection|GetTargetLocation) (Transformation|GetWorldLocation (Variables|Default|GetTowerTop)))))))) _returnvalue _s_rotation_speed) false false)
                (Transformation|SetRelativeRotation (Variables|Default|GetTowerTop) (Class|KismetMathLibrary|RInterptoConstant (Variables|/Script/Engine.SceneComponent|GetRelativeRotation (Variables|Default|GetTowerTop)) (Math|Rotator|MakeRotator 0.0 (.Pitch (Math|Rotator|BreakRotator (Math|Rotator|MakeRotfromX (Math|Transform|InverseTransformDirection (Transformation|GetActorTransform) (- (Variables|TargetDetection|GetTargetLocation) (Transformation|GetWorldLocation (Variables|Default|GetTowerTop))))))) 0.0) _returnvalue _s_rotation_speed) false false)
                (Utilities|IsValid (Variables|TargetDetection|GetTarget)
                  (:Is%20Valid
                    (bind _result (CallFunction|SightOfTarget (Transformation|GetWorldLocation (Variables|Default|GetArrow)) (Transformation|GetActorLocation (Variables|TargetDetection|GetTarget)) (Utilities|Array|MakeArray self (Variables|TargetDetection|GetTarget))))
                    (if _result
                      (CallFunction|UpdateFire)
                      (else
                        (CallFunction|Stop)))
                    (Utilities|FlowControl|Delay (Utilities|Time|GetWorldDeltaSeconds))
                    (CallFunction|ContinueAim))))
              (:Is%20Not%20Valid
                (CallFunction|CancelAim :!label _label)
                (CallFunction|StartReset)))))))
    (:Is%20Not%20Valid
      (if (not _withered)
        (goto _label)))))

(event EventBeginPlay
  (Components|Sphere|SetSphereRadius (Variables|Default|GetSphere) (Variables|Upgrade|GetS%20Tower%20Range) true)
  (Utilities|Time|SetTimerbyEvent (EventDispatchers|CreateEvent :!event Custom|HydrationEvent) 1.0 true))

(event EventWater
  (params (Amount :type Float%20%28double-precision%29))
  ;[1 1 1] Allow the player to hydrate the tower, recovering it from a withered state.
  (Utilities|FlowControl|Delay 0.1)
  (Variables|Default|SetHydration (Math|Integer|Clamp(Integer) (Math|Float|Truncate (+ Amount (Variables|Default|GetHydration))) 0 100))
  (Variables|Default|SetWithered false)
  ;[1 1 1] Check if anything is inside the range after watering.
  (for _array_element (Collision|GetOverlappingActors (Variables|Default|GetSphere) "/Game/Tech/Enemies/BP_BaseEnemy.BP_BaseEnemy_C" :!class /Script/Engine.PrimitiveComponent)
    (bind _asbp_base_enemy (Utilities|Casting|CastToBP_BaseEnemy _array_element))
    (Utilities|Array|Add (Variables|TargetDetection|GetEnemiesInRange) _asbp_base_enemy))
  (CallFunction|SelectTarget)
  (Rendering|Components|TextRender|SetText (Variables|Default|GetTextRender) (Utilities|Text|ToText(Integer) (Variables|Default|GetHydration))))

(event EventTick
  (params (DeltaSeconds :type Float%20%28single-precision%29))
  (if (Variables|Default|GetWithered)
    _))

(fn ConstructionScript)

(fn UpdateFire
  ;[1 1 1] Cooldown for Firing
  (if (> (- (Utilities|Time|GetGameTimeinSeconds) (Variables|Default|GetLast%20Time%20Tower%20Fired)) (Variables|Upgrade|GetS%20Fire%20Rate))
    (if (> (Math|Vector|DotProduct (Math|Vector|GetUnitDirection(Vector) (Transformation|GetWorldLocation (Variables|Default|GetArrow)) (Transformation|GetActorLocation (Variables|TargetDetection|GetTarget))) (Math|Vector|GetForwardVector (Variables|Default|GetArrow))) 0.99999) ; Turret Facing Target
      (CallFunction|Fire))))