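; Test broccoli tower Blueprint that stops enemies entering its growth area, extending inherited base tower logic.
; Every tick, it repositions GrowthMesh below the Tower component, dropping it lower when Hydration runs out.
; GrowthMesh overlaps set BP_BaseEnemy speed to zero.
; End overlap assigns each enemy's speed to itself, so the original speed is not restored here.
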(event OnComponentBeginOverlap(GrowthMesh)
  (params (OverlappedComponent :type Primitive%20Component%20Object%20Reference) (OtherActor :type Actor%20Object%20Reference) (OtherComp :type Primitive%20Component%20Object%20Reference) (OtherBodyIndex :type Integer) (bFromSweep :type Boolean) (SweepResult :type Hit%20Result%20Structure%20%28by%20ref%29))
  (bind _asbp_base_enemy (Utilities|Casting|CastToBP_BaseEnemy OtherActor))
  (Variables|/Game/Tech/Enemies/BP_BaseEnemy.BP_BaseEnemy_C|SetSpeed _asbp_base_enemy 0.0))

(event OnComponentEndOverlap(GrowthMesh)
  (params (OverlappedComponent :type Primitive%20Component%20Object%20Reference) (OtherActor :type Actor%20Object%20Reference) (OtherComp :type Primitive%20Component%20Object%20Reference) (OtherBodyIndex :type Integer))
  (bind _asbp_base_enemy (Utilities|Casting|CastToBP_BaseEnemy OtherActor))
  (Variables|/Game/Tech/Enemies/BP_BaseEnemy.BP_BaseEnemy_C|SetSpeed _asbp_base_enemy (Variables|/Game/Tech/Enemies/BP_BaseEnemy.BP_BaseEnemy_C|GetSpeed _asbp_base_enemy)))

(event Custom|AOECheck
  (bind _growth_mesh (Variables|Default|GetGrowth%20Mesh))
  (if (<= (Variables|Default|GetHydration) 0)
    (Transformation|SetRelativeLocation _growth_mesh (+ (Variables|/Script/Engine.SceneComponent|GetRelativeLocation (Variables|Default|GetTower)) "0.000000,0.000000,-160.000000") false false)
    (else
      (Transformation|SetRelativeLocation _growth_mesh (+ (Variables|/Script/Engine.SceneComponent|GetRelativeLocation (Variables|Default|GetTower)) "0.000000,0.000000,-125.000000") false false))))

(event EventBeginPlay
  (|CallParentFunction))

(event EventTick
  (params (DeltaSeconds :type Float%20%28single-precision%29))
  (|CallParentFunction DeltaSeconds)
  (CallFunction|AOECheck))

(event Collision|EventActorBeginOverlap
  (params (OtherActor :type Actor%20Object%20Reference)))

(fn ConstructionScript
  (|CallParentFunction))