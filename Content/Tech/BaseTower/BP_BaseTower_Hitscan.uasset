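; Hitscan tower that automatically targets and shoots pawns within its range.
; Each tick it picks the closest pawn that passes a line-of-sight check, then turns the tower top toward it at constant speed.
; Once the cooldown has elapsed and a dot-product test confirms aim, Fire runs a delayed DoN loop for burst shots.
; Each shot line-traces from the arrow to the target, damages the hit actor and leaves a persistent debug line.
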(event Custom|Fire
  (Variables|Private|SetLast%20Time%20Tower%20Fired (Utilities|Time|GetGameTimeinSeconds))
  (Utilities|FlowControl|Sequence
    (:then_0
      (goto _label Reset))
    (:then_1
      (Utilities|FlowControl|DoN (Variables|Default|GetFireHowManyAtOnce) :!label _label
        (:Exit
          (bind _outhit (Collision|LineTraceByChannel (.location (Transformation|GetWorldTransform (Variables|Default|GetArrow))) (Transformation|GetActorLocation (Variables|Private|GetTarget)) "TraceTypeQuery1" false 0 "Persistent"))
          (Development|PrintString "Hit" false)
          (Game|Damage|ApplyDamage (.hitactor _outhit) (Variables|Default|GetTower%20Hitscan%20Damage) 0 0)
          (Utilities|FlowControl|Delay 0.1)
          (goto _label))))))

(event EventTick
  (params (DeltaSeconds :type Float%20%28single-precision%29))
  (CallFunction|FindTarget)
  (Variables|Private|GetTarget
    (:then
      (CallFunction|RotateTowerTop DeltaSeconds)
      (CallFunction|UpdateFire))
    (:else)))

(fn ConstructionScript)

(fn FindTarget
  (LocalVariables|SetBestDistance (+ (Variables|Upgrades|GetTowerRange) 1.0))
  (bind _outactors (Collision|SphereOverlapActors (Transformation|GetActorLocation) (Variables|Upgrades|GetTowerRange) (Utilities|Array|MakeArray "ObjectTypeQuery3") "/Script/Engine.Actor"))
  (for _array_element _outactors
    (bind _output_get (LocalVariables|SetCurrentTarget _array_element))
    (bind _output_get_2 (LocalVariables|SetCurrentDistance (Transformation|GetDistanceTo _output_get self)))
    (if (or (< _output_get_2 (LocalVariables|GetBestDistance)) (not (Utilities|IsValid (LocalVariables|GetBestTarget)))) ; Closest Target
      (bind _result (CallFunction|SightOfTarget (Transformation|GetWorldLocation (Variables|Default|GetTowerTop)) (Transformation|GetActorLocation (LocalVariables|GetCurrentTarget)) (Utilities|Array|MakeArray self (LocalVariables|GetCurrentTarget))))
      (if _result
        (LocalVariables|SetBestTarget (LocalVariables|GetCurrentTarget))
        (LocalVariables|SetBestDistance (LocalVariables|GetCurrentDistance)))))
  (Variables|Private|SetTarget (LocalVariables|GetBestTarget)))

(fn RotateTowerTop
  (params (Delta%20Seconds :type Float%20%28double-precision%29))
  (Transformation|SetWorldRotation (Variables|Default|GetTowerTop) (Class|KismetMathLibrary|RInterptoConstant (Transformation|GetWorldRotation (Variables|Default|GetTowerTop)) (Math|Rotator|FindLookatRotation (Transformation|GetWorldLocation (Variables|Default|GetTowerTop)) (Transformation|GetActorLocation (Variables|Private|GetTarget))) Delta%20Seconds (Variables|Upgrades|GetRotationSpeed)) false false))

(fn UpdateFire
  ;[1 1 1] Cooldown for Firing
  (if (> (- (Utilities|Time|GetGameTimeinSeconds) (Variables|Private|GetLast%20Time%20Tower%20Fired)) (Variables|Upgrades|GetFireRate))
    (if (> (Math|Vector|DotProduct (Math|Vector|GetUnitDirection(Vector) (Transformation|GetWorldLocation (Variables|Default|GetTowerTop)) (Transformation|GetActorLocation (Variables|Private|GetTarget))) (Math|Vector|GetForwardVector (Variables|Default|GetTowerTop))) 0.99999) ; Turret Facing Target
      (CallFunction|Fire))))