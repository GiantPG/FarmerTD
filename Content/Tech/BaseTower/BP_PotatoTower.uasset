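; Potato Tower, a tower Blueprint that attacks its target with area-of-effect projectiles.
; It sets its display name on BeginPlay and extends the parent's FireFunction, recording the time of each shot.
; A DoN node, reset and entered on each call, gates spawning of BP_Projectile_AOE at the Arrow's transform when the target is valid, passing damage from TowerStats.
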(event EventBeginPlay
  (Variables|Default|SetName "Potato Tower")
  (|CallParentFunction))

(event Collision|EventActorBeginOverlap
  (params (OtherActor :type Actor%20Object%20Reference)))

(event EventTick
  (params (DeltaSeconds :type Float%20%28single-precision%29))
  (|CallParentFunction DeltaSeconds) ; This node is disabled and will not be called.\nDrag off pins to build functionality.
)

(fn ConstructionScript
  (|CallParentFunction))

(fn FireFunction
  (bind _arrow (Variables|Default|GetArrow))
  (bind _returnvalue (Transformation|GetWorldTransform _arrow))
  (|CallParentFunction)
  (Variables|Default|SetLast%20Time%20Tower%20Fired (Utilities|Time|GetGameTimeinSeconds))
  (Utilities|FlowControl|Sequence
    (:then_0
      (goto _label Reset))
    (:then_1
      (Utilities|FlowControl|DoN (Variables|Default|GetFireHowManyAtOnce) :!label _label
        (:Exit
          (Utilities|IsValid (Variables|Default|GetTarget)
            (:Is%20Valid
              (Game|SpawnActorfromClass "/Game/Tech/BaseProjectile/BP_Projectile_AOE.BP_Projectile_AOE_C" (Math|Transform|MakeTransform (.location _returnvalue) (.rotation _returnvalue) "1.000000,1.000000,1.000000") "Undefined" self (.damage (Variables|Default|GetTowerStats)) 0))))))))