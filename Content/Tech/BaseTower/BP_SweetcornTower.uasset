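; Sweetcorn Tower is a tower Blueprint that fires randomly spread hitscan shots at its target.
; Its FireFunction extends the parent's, records the fire time, then resets and enters a DoN, producing one trace per call.
; The trace runs from the Arrow toward the offset target location, damaging the hit actor using TowerStats, with debug line and print.
; An unconnected EventGraph copy repeats shots on a short delay.
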(event EventBeginPlay
  (Variables|Default|SetName "Sweetcorn Tower")
  (|CallParentFunction))

(event Collision|EventActorBeginOverlap
  (params (OtherActor :type Actor%20Object%20Reference)))

(event EventTick
  (params (DeltaSeconds :type Float%20%28single-precision%29))
  (|CallParentFunction DeltaSeconds) ; This node is disabled and will not be called.\nDrag off pins to build functionality.
)

(fn ConstructionScript
  (|CallParentFunction))

(fn FireFunction
  (bind _min_spread (Variables|Default|GetMin%20Spread))
  (bind _max_spread (Variables|Default|GetMax%20Spread))
  (bind _target (Variables|Default|GetTarget))
  (bind _returnvalue (Transformation|GetActorLocation _target))
  (|CallParentFunction)
  (Variables|Default|SetLast%20Time%20Tower%20Fired (Utilities|Time|GetGameTimeinSeconds))
  (Utilities|FlowControl|Sequence
    (:then_0
      (goto _label Reset))
    (:then_1
      (Utilities|FlowControl|DoN (Variables|Default|GetFireHowManyAtOnce) :!label _label
        (:Exit
          (Utilities|IsValid (Variables|Default|GetTarget)
            (:Is%20Valid
              (bind _outhit (Collision|LineTraceByChannel (.location (Transformation|GetWorldTransform (Variables|Default|GetArrow))) (Math|Vector|MakeVector (+ (.x _returnvalue) (Math|Random|RandomFloatinRange _min_spread _max_spread)) (+ (.y _returnvalue) (Math|Random|RandomFloatinRange _min_spread _max_spread)) (+ (.z _returnvalue) (Math|Random|RandomFloatinRange _min_spread _max_spread))) "TraceTypeQuery1" false 0 "Persistent"))
              (Development|PrintString "Hit" false)
              (Game|Damage|ApplyDamage (.hitactor _outhit) (.damage (Variables|Default|GetTowerStats)) 0 0))))))))