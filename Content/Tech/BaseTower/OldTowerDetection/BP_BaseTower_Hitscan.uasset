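; Hitscan defense tower that shoots enemies and withers, going inactive, when its Hydration runs out; TransferWater refills it.
; Each Tick, FindTarget seeks the closest enemy in range with line of sight, and RotateTowerTop turns toward it at constant speed.
; UpdateFire gates Fire by cooldown and a dot-product aim check; Fire uses DoN for delayed line-trace damage bursts.
; Three identical upgrade events multiply damage, rotation, fire rate and range.
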(event Custom|Fire
  (Variables|Private|SetLast%20Time%20Tower%20Fired (Utilities|Time|GetGameTimeinSeconds))
  (Utilities|FlowControl|Sequence
    (:then_0
      (goto _label Reset))
    (:then_1
      (Utilities|FlowControl|DoN (Variables|Default|GetFireHowManyAtOnce) :!label _label
        (:Exit
          (bind _outhit (Collision|LineTraceByChannel (.location (Transformation|GetWorldTransform (Variables|Default|GetArrow))) (Transformation|GetActorLocation (Variables|Private|GetTarget)) "TraceTypeQuery1" false 0 "Persistent"))
          (Development|PrintString "Hit" false)
          (Game|Damage|ApplyDamage (.hitactor _outhit) (Variables|Default|GetTower%20Hitscan%20Damage) 0 0)
          (Utilities|FlowControl|Delay 0.1)
          (goto _label))))))

(event Custom|Upgrade%20LVL1
  (Variables|Upgrade|SetS%20Damage (* (Variables|Upgrade|GetS%20Damage) 1.3))
  (Variables|Upgrade|SetS%20Rotation%20Speed (* (Variables|Upgrade|GetS%20Rotation%20Speed) 1.2))
  (Variables|Upgrade|SetS%20Fire%20Rate (* (Variables|Upgrade|GetS%20Fire%20Rate) -0.5))
  (Variables|Upgrade|SetS%20Tower%20Range (* (Variables|Upgrade|GetS%20Tower%20Range) 1.2)))

(event Custom|HydrationEvent
  ;[1 1 1] Drain Hydration
  (bind _output_get (Variables|Default|SetHydration (Math|Integer|Clamp(Integer) (- (Variables|Default|GetHydration) 1) 0 100)))
  (if (<= _output_get 0)
    (Variables|Default|SetWithered true))
  (Rendering|Components|TextRender|SetText (Variables|Default|GetTextRender) (Utilities|Text|ToText(Integer) (Variables|Default|GetHydration))))

(event Custom|Upgrade%20LVL3
  (Variables|Upgrade|SetS%20Damage (* (Variables|Upgrade|GetS%20Damage) 1.3))
  (Variables|Upgrade|SetS%20Rotation%20Speed (* (Variables|Upgrade|GetS%20Rotation%20Speed) 1.2))
  (Variables|Upgrade|SetS%20Fire%20Rate (* (Variables|Upgrade|GetS%20Fire%20Rate) -0.5))
  (Variables|Upgrade|SetS%20Tower%20Range (* (Variables|Upgrade|GetS%20Tower%20Range) 1.2)))

(event Custom|Upgrade%20LVL2
  (Variables|Upgrade|SetS%20Damage (* (Variables|Upgrade|GetS%20Damage) 1.3))
  (Variables|Upgrade|SetS%20Rotation%20Speed (* (Variables|Upgrade|GetS%20Rotation%20Speed) 1.2))
  (Variables|Upgrade|SetS%20Fire%20Rate (* (Variables|Upgrade|GetS%20Fire%20Rate) -0.5))
  (Variables|Upgrade|SetS%20Tower%20Range (* (Variables|Upgrade|GetS%20Tower%20Range) 1.2)))

(event EventBeginPlay
  (Variables|Upgrade|SetS%20Damage (Variables|Upgrade|GetS%20Damage))
  (Variables|Upgrade|SetS%20Tower%20Range (Variables|Upgrade|GetS%20Tower%20Range))
  (Variables|Upgrade|SetS%20Fire%20Rate (Variables|Upgrade|GetS%20Fire%20Rate))
  (Utilities|Time|SetTimerbyEvent (EventDispatchers|CreateEvent :!event Custom|HydrationEvent) 1.0 true))

(event EventTransferWater
  (params (Amount :type Float%20%28double-precision%29))
  (Utilities|FlowControl|Delay 0.1)
  (Variables|Default|SetHydration (Math|Integer|Clamp(Integer) (Math|Float|Truncate (+ Amount (Variables|Default|GetHydration))) 0 100))
  (Variables|Default|SetWithered false)
  (Rendering|Components|TextRender|SetText (Variables|Default|GetTextRender) (Utilities|Text|ToText(Integer) (Variables|Default|GetHydration))))

(event EventTick
  (params (DeltaSeconds :type Float%20%28single-precision%29))
  (if (not (Variables|Default|GetWithered))
    (CallFunction|FindTarget)
    (Variables|Private|GetTarget
      (:then
        (CallFunction|RotateTowerTop DeltaSeconds)
        (CallFunction|UpdateFire))
      (:else))))

(fn ConstructionScript)

(fn FindTarget
  (LocalVariables|SetBestDistance (+ (Variables|Upgrade|GetS%20Tower%20Range) 1.0))
  (bind _outactors (Collision|SphereOverlapActors (Transformation|GetActorLocation) (Variables|Upgrade|GetS%20Tower%20Range) (Utilities|Array|MakeArray "ObjectTypeQuery3") "/Game/Tech/Enemies/BP_BaseEnemy.BP_BaseEnemy_C"))
  (for _array_element _outactors
    (bind _output_get (LocalVariables|SetCurrentTarget _array_element))
    (if (<= (Math|Vector|Distance(Vector) (Transformation|GetActorLocation _output_get) (Transformation|GetActorLocation)) (LocalVariables|GetBestDistance)) ; Closest Target
      (bind _result (CallFunction|SightOfTarget (Transformation|GetWorldLocation (Variables|Default|GetTowerTop)) (Transformation|GetActorLocation (LocalVariables|GetCurrentTarget)) (Utilities|Array|MakeArray self (LocalVariables|GetCurrentTarget))))
      (if _result
        (LocalVariables|SetBestTarget (LocalVariables|GetCurrentTarget))
        (LocalVariables|SetBestDistance (LocalVariables|GetCurrentDistance)))))
  (Variables|Private|SetTarget (LocalVariables|GetBestTarget)))

(fn RotateTowerTop
  (params (Delta%20Seconds :type Float%20%28double-precision%29))
  (Transformation|SetWorldRotation (Variables|Default|GetTowerTop) (Class|KismetMathLibrary|RInterptoConstant (Transformation|GetWorldRotation (Variables|Default|GetTowerTop)) (Math|Rotator|FindLookatRotation (Transformation|GetWorldLocation (Variables|Default|GetTowerTop)) (Transformation|GetActorLocation (Variables|Private|GetTarget))) Delta%20Seconds (Variables|Upgrade|GetS%20Rotation%20Speed)) false false))

(fn UpdateFire
  ;[1 1 1] Cooldown for Firing
  (if (> (- (Utilities|Time|GetGameTimeinSeconds) (Variables|Private|GetLast%20Time%20Tower%20Fired)) (Variables|Upgrade|GetS%20Fire%20Rate))
    (if (> (Math|Vector|DotProduct (Math|Vector|GetUnitDirection(Vector) (Transformation|GetWorldLocation (Variables|Default|GetTowerTop)) (Transformation|GetActorLocation (Variables|Private|GetTarget))) (Math|Vector|GetForwardVector (Variables|Default|GetTowerTop))) 0.99999) ; Turret Facing Target
      (CallFunction|Fire))))