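; Growth variant of the base tower, with a water-fed growth mesh that sets overlapping enemies' speed.
; Water raises Hydration and a looping timer drains it, with the mesh sitting lower once dry.
; Tick finds a visible enemy in range by sphere overlap and sight check, then rotates the top toward it.
; Three identical upgrade events scale stats, while firing is unfinished: UpdateFire is never called and Fire is disconnected.
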(event OnComponentBeginOverlap(GrowthMesh)
  (params (OverlappedComponent :type Primitive%20Component%20Object%20Reference) (OtherActor :type Actor%20Object%20Reference) (OtherComp :type Primitive%20Component%20Object%20Reference) (OtherBodyIndex :type Integer) (bFromSweep :type Boolean) (SweepResult :type Hit%20Result%20Structure%20%28by%20ref%29))
  (bind _asbp_base_enemy (Utilities|Casting|CastToBP_BaseEnemy OtherActor))
  (Variables|/Game/Tech/Enemies/BP_BaseEnemy.BP_BaseEnemy_C|SetSpeed _asbp_base_enemy 2.5e+02))

(event Custom|HydrationEvent
  ;[1 1 1] Drain Hydration
  (bind _output_get (Variables|Default|SetHydration (Math|Integer|Clamp(Integer) (- (Variables|Default|GetHydration) 1) 0 100)))
  (if (<= _output_get 0)
    (Variables|Default|SetWithered true)
    (CallFunction|AOECheck))
  (Rendering|Components|TextRender|SetText (Variables|Default|GetTextRender) (Utilities|Text|ToText(Integer) (Variables|Default|GetHydration))))

(event Custom|Upgrade%20LVL1
  (Variables|Upgrades|SetS%20Damage (* (Variables|Upgrades|GetS%20Damage) 1.3))
  (Variables|Upgrades|SetS%20Rotation%20Speed (* (Variables|Upgrades|GetS%20Rotation%20Speed) 1.2))
  (Variables|Upgrades|SetS%20Fire%20Rate (* (Variables|Upgrades|GetS%20Fire%20Rate) -0.5))
  (Variables|Upgrades|SetS%20Tower%20Range (* (Variables|Upgrades|GetS%20Tower%20Range) 1.2)))

(event Custom|AOECheck
  (bind _growthmesh (Variables|Default|GetGrowthMesh))
  (if (<= (Variables|Default|GetHydration) 0)
    (Transformation|SetRelativeLocation _growthmesh (+ (Variables|/Script/Engine.SceneComponent|GetRelativeLocation (Variables|Default|GetTower)) "0.000000,0.000000,-160.000000") false false)
    (else
      (Transformation|SetRelativeLocation _growthmesh (+ (Variables|/Script/Engine.SceneComponent|GetRelativeLocation (Variables|Default|GetTower)) "0.000000,0.000000,-125.000000") false false))))

(event Custom|Upgrade%20LVL2
  (Variables|Upgrades|SetS%20Damage (* (Variables|Upgrades|GetS%20Damage) 1.3))
  (Variables|Upgrades|SetS%20Rotation%20Speed (* (Variables|Upgrades|GetS%20Rotation%20Speed) 1.2))
  (Variables|Upgrades|SetS%20Fire%20Rate (* (Variables|Upgrades|GetS%20Fire%20Rate) -0.5))
  (Variables|Upgrades|SetS%20Tower%20Range (* (Variables|Upgrades|GetS%20Tower%20Range) 1.2)))

(event Custom|Upgrade%20LVL3
  (Variables|Upgrades|SetS%20Damage (* (Variables|Upgrades|GetS%20Damage) 1.3))
  (Variables|Upgrades|SetS%20Rotation%20Speed (* (Variables|Upgrades|GetS%20Rotation%20Speed) 1.2))
  (Variables|Upgrades|SetS%20Fire%20Rate (* (Variables|Upgrades|GetS%20Fire%20Rate) -0.5))
  (Variables|Upgrades|SetS%20Tower%20Range (* (Variables|Upgrades|GetS%20Tower%20Range) 1.2)))

(event EventBeginPlay
  (Variables|Upgrades|SetS%20Damage (Variables|Upgrades|GetS%20Damage))
  (Variables|Upgrades|SetS%20Tower%20Range (Variables|Upgrades|GetS%20Tower%20Range))
  (Variables|Upgrades|SetS%20Fire%20Rate (Variables|Upgrades|GetS%20Fire%20Rate))
  (CallFunction|AOECheck)
  (Utilities|Time|SetTimerbyEvent (EventDispatchers|CreateEvent :!event Custom|HydrationEvent) 1.0 true))

(event EventWater
  (params (Amount :type Float%20%28double-precision%29))
  (Utilities|FlowControl|Delay 0.1)
  (Variables|Default|SetHydration (Math|Integer|Clamp(Integer) (Math|Float|Truncate (+ Amount (Variables|Default|GetHydration))) 0 100))
  (CallFunction|AOECheck)
  (Rendering|Components|TextRender|SetText (Variables|Default|GetTextRender) (Utilities|Text|ToText(Integer) (Variables|Default|GetHydration))))

(event EventTick
  (params (DeltaSeconds :type Float%20%28single-precision%29))
  (CallFunction|FindTarget)
  (Variables|Private|GetTarget
    (:then
      (CallFunction|RotateTowerTop DeltaSeconds))
    (:else)))

(fn ConstructionScript)

(fn FindTarget
  (LocalVariables|SetBestDistance (+ (Variables|Upgrades|GetS%20Tower%20Range) 1.0))
  (bind _outactors (Collision|SphereOverlapActors (Transformation|GetActorLocation) (Variables|Upgrades|GetS%20Tower%20Range) (Utilities|Array|MakeArray "ObjectTypeQuery3") "/Game/Tech/Enemies/BP_BaseEnemy.BP_BaseEnemy_C"))
  (for _array_element _outactors
    (bind _output_get (LocalVariables|SetCurrentTarget _array_element))
    (if (<= (Math|Vector|Distance(Vector) (Transformation|GetActorLocation _output_get) (Transformation|GetActorLocation)) (LocalVariables|GetBestDistance)) ; Closest Target
      (bind _result (CallFunction|SightOfTarget (Transformation|GetWorldLocation (Variables|Default|GetTowerTop)) (Transformation|GetActorLocation (LocalVariables|GetCurrentTarget)) (Utilities|Array|MakeArray self (LocalVariables|GetCurrentTarget))))
      (if _result
        (LocalVariables|SetBestTarget (LocalVariables|GetCurrentTarget))
        (LocalVariables|SetBestDistance (LocalVariables|GetCurrentDistance)))))
  (Variables|Private|SetTarget (LocalVariables|GetBestTarget)))

(fn RotateTowerTop
  (params (Delta%20Seconds :type Float%20%28double-precision%29))
  (Transformation|SetWorldRotation (Variables|Default|GetTowerTop) (Class|KismetMathLibrary|RInterptoConstant (Transformation|GetWorldRotation (Variables|Default|GetTowerTop)) (Math|Rotator|FindLookatRotation (Transformation|GetWorldLocation (Variables|Default|GetTowerTop)) (Transformation|GetActorLocation (Variables|Private|GetTarget))) Delta%20Seconds (Variables|Upgrades|GetS%20Rotation%20Speed)) false false))

(fn UpdateFire
  ;[1 1 1] Cooldown for Firing
  (if (> (- (Utilities|Time|GetGameTimeinSeconds) (Variables|Private|GetLast%20Time%20Tower%20Fired)) (Variables|Upgrades|GetS%20Fire%20Rate))
    (if (> (Math|Vector|DotProduct (Math|Vector|GetUnitDirection(Vector) (Transformation|GetWorldLocation (Variables|Default|GetTowerTop)) (Transformation|GetActorLocation (Variables|Private|GetTarget))) (Math|Vector|GetForwardVector (Variables|Default|GetTowerTop))) 0.99999) ; Turret Facing Target
      _)))