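; Carrot Tower, a child tower that sets its display name on BeginPlay and fires hitscan shots at its target.
; Its FireFunction runs the parent logic, records the fire time, then line-traces from the Arrow to a valid Target and applies TowerStats damage to the actor hit.
; The DoN gate sized by FireHowManyAtOnce is reset and entered once per call, so each call fires one trace, drawn with persistent debug lines.
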(event EventBeginPlay
  (Variables|Default|SetName "Carrot Tower")
  (|CallParentFunction))

(event Collision|EventActorBeginOverlap
  (params (OtherActor :type Actor%20Object%20Reference)))

(event EventTick
  (params (DeltaSeconds :type Float%20%28single-precision%29))
  (|CallParentFunction DeltaSeconds) ; This node is disabled and will not be called.\nDrag off pins to build functionality.
)

(fn ConstructionScript
  (|CallParentFunction))

(fn FireFunction
  (|CallParentFunction)
  (Variables|Default|SetLast%20Time%20Tower%20Fired (Utilities|Time|GetGameTimeinSeconds))
  (Utilities|FlowControl|Sequence
    (:then_0
      (goto _label Reset))
    (:then_1
      (Utilities|FlowControl|DoN (Variables|Default|GetFireHowManyAtOnce) :!label _label
        (:Exit
          (Utilities|IsValid (Variables|Default|GetTarget)
            (:Is%20Valid
              (bind _outhit (Collision|LineTraceByChannel (.location (Transformation|GetWorldTransform (Variables|Default|GetArrow))) (Transformation|GetActorLocation (Variables|Default|GetTarget)) "TraceTypeQuery1" false 0 "Persistent"))
              (Game|Damage|ApplyDamage (.hitactor _outhit) (.damage (Variables|Default|GetTowerStats)) 0 self))))))))