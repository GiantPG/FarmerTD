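; Melee test tower named "Dragon Fruit Tower" that extends a parent tower and attacks by stabbing with a blade.
; Fire records the time, then resets and enters a DoN that repeats the stab up to FireHowManyAtOnce times while Target is valid.
; Each stab jumps the Blade out and back with short delays and no sweep, as the Lerps have zero alpha.
; Separately, any Capsule overlap applies SDamage and prints a debug message.
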(event OnComponentBeginOverlap(Capsule)
  (params (OverlappedComponent :type Primitive%20Component%20Object%20Reference) (OtherActor :type Actor%20Object%20Reference) (OtherComp :type Primitive%20Component%20Object%20Reference) (OtherBodyIndex :type Integer) (bFromSweep :type Boolean) (SweepResult :type Hit%20Result%20Structure%20%28by%20ref%29))
  (Game|Damage|ApplyDamage OtherActor (Variables|Default|GetS%20Damage) 0 0)
  (Development|PrintString "Stabby Stab!"))

(event EventBeginPlay
  (Variables|Default|SetName "Dragon Fruit Tower")
  (|CallParentFunction))

(event Collision|EventActorBeginOverlap
  (params (OtherActor :type Actor%20Object%20Reference)))

(event EventTick
  (params (DeltaSeconds :type Float%20%28single-precision%29))
  (|CallParentFunction DeltaSeconds) ; This node is disabled and will not be called.\nDrag off pins to build functionality.
)

(event EventFire
  (Variables|Default|SetLast%20Time%20Tower%20Fired (Utilities|Time|GetGameTimeinSeconds))
  (Utilities|FlowControl|Sequence
    (:then_0
      (goto _label Reset))
    (:then_1
      (Utilities|FlowControl|DoN (Variables|Default|GetFireHowManyAtOnce) :!label _label
        (:Exit
          (Utilities|IsValid (Variables|Default|GetTarget)
            (:Is%20Valid
              (Transformation|AddRelativeLocation (Variables|Default|GetBlade) (Math|Vector|Lerp(Vector) (Variables|Default|GetA) "0, 0, 0" 0.0) false false)
              (Utilities|FlowControl|Delay 0.2)
              (Transformation|AddRelativeLocation (Variables|Default|GetBlade) (Math|Vector|Lerp(Vector) (* (Variables|Default|GetA) -1.0) "0, 0, 0" 0.0) false false)
              (Utilities|FlowControl|Delay 0.1)
              (goto _label))))))))

(fn ConstructionScript
  (|CallParentFunction))