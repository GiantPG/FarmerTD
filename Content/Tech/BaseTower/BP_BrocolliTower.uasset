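; Broccoli tower, a child of a base tower, that slows actors inside the area covered by its growth mesh.
; GrowthMesh overlaps send a slow message using the TowerStats slow effect, then a restore-speed message on exit.
; AOECheck, called at BeginPlay, waits briefly, then drops the mesh far below the tower when Hydration is depleted or places it slightly above otherwise.
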(event OnComponentBeginOverlap(GrowthMesh)
  (params (OverlappedComponent :type Primitive%20Component%20Object%20Reference) (OtherActor :type Actor%20Object%20Reference) (OtherComp :type Primitive%20Component%20Object%20Reference) (OtherBodyIndex :type Integer) (bFromSweep :type Boolean) (SweepResult :type Hit%20Result%20Structure%20%28by%20ref%29))
  (Class|BPITargettable|Slow(Message) OtherActor (.sloweffect (Variables|Default|GetTowerStats))))

(event OnComponentEndOverlap(GrowthMesh)
  (params (OverlappedComponent :type Primitive%20Component%20Object%20Reference) (OtherActor :type Actor%20Object%20Reference) (OtherComp :type Primitive%20Component%20Object%20Reference) (OtherBodyIndex :type Integer))
  (Class|BPITargettable|RestoreSpeed(Message) OtherActor))

(event Custom|AOECheck
  (bind _growth_mesh (Variables|Default|GetGrowth%20Mesh))
  (Utilities|FlowControl|Delay 0.001)
  (if (<= (Variables|Default|GetHydration) 0.0)
    (Transformation|SetRelativeLocation _growth_mesh (+ (Variables|/Script/Engine.SceneComponent|GetRelativeLocation (Variables|Default|GetTower)) "0.000000,0.000000,-270.000000") false false)
    (else
      (Transformation|SetRelativeLocation _growth_mesh (+ (Variables|/Script/Engine.SceneComponent|GetRelativeLocation (Variables|Default|GetTower)) "0.000000,0.000000,10.000000") false false))))

(event EventBeginPlay
  (Variables|Default|SetName "Broccoli Tower")
  (|CallParentFunction)
  (CallFunction|AOECheck))

(event EventTick
  (params (DeltaSeconds :type Float%20%28single-precision%29))
  (|CallParentFunction DeltaSeconds))

(event Collision|EventActorBeginOverlap
  (params (OtherActor :type Actor%20Object%20Reference)))

(fn ConstructionScript
  (|CallParentFunction))