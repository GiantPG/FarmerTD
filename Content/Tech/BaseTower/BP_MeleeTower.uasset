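; BP_MeleeTower is the "Dragon Fruit Tower", a child tower that attacks with a swinging sword.
; FireFunction records the fire time and calls SwordSwing through a self-re-entering DoN while Target is valid.
; A timeline rotates SwordHandle forward, then reverses it.
; Box1 overlaps apply TowerStats.Damage through a DoOnce gate, which the timeline resets on every update above 0.3 alpha.
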(event OnComponentBeginOverlap(Box1)
  (params (OverlappedComponent :type Primitive%20Component%20Object%20Reference) (OtherActor :type Actor%20Object%20Reference) (OtherComp :type Primitive%20Component%20Object%20Reference) (OtherBodyIndex :type Integer) (bFromSweep :type Boolean) (SweepResult :type Hit%20Result%20Structure%20%28by%20ref%29))
  (Utilities|FlowControl|DoOnce false
    (:Completed
      (Game|Damage|ApplyDamage OtherActor (.damage (Variables|Default|GetTowerStats)) 0 self)
      (Development|PrintString "Stabby Stab!"))))

(event Custom|SwordSwing
  (bind (_direction _newtrack_0) (Timeline|SwordSwingTimeline PlayFromStart)
    (:Update
      (Transformation|SetRelativeRotation (Variables|Default|GetSwordHandle) (Math|Rotator|Lerp(Rotator) "90.000000,90.000000,90.000000" "0.000000,90.000000,90.000000" _newtrack_0 true) false false)
      (if (> _newtrack_0 0.3)
        (CallFunction|ResetLethality)))
    (:Finished
      (switch Utilities|FlowControl|Switch|SwitchonETimelineDirection _direction
        (:Forward
          (CallFunction|ResetSwing))))))

(event Custom|ResetSwing
  (bind (_direction _newtrack_0) (Timeline|SwordSwingTimeline ReverseFromEnd)
    (:Update
      (Transformation|SetRelativeRotation (Variables|Default|GetSwordHandle) (Math|Rotator|Lerp(Rotator) "90.000000,90.000000,90.000000" "0.000000,90.000000,90.000000" _newtrack_0 true) false false)
      (if (> _newtrack_0 0.3)
        (CallFunction|ResetLethality)))
    (:Finished
      (switch Utilities|FlowControl|Switch|SwitchonETimelineDirection _direction
        (:Forward
          (CallFunction|ResetSwing))))))

(event Custom|ResetLethality
  (Utilities|FlowControl|DoOnce false) ; enters at Reset
)

(event EventBeginPlay
  (Variables|Default|SetName "Dragon Fruit Tower")
  (|CallParentFunction))

(event Collision|EventActorBeginOverlap
  (params (OtherActor :type Actor%20Object%20Reference)))

(event EventTick
  (params (DeltaSeconds :type Float%20%28single-precision%29))
  (|CallParentFunction DeltaSeconds) ; This node is disabled and will not be called.\nDrag off pins to build functionality.
)

(fn ConstructionScript
  (|CallParentFunction))

(fn FireFunction
  (|CallParentFunction)
  (Variables|Default|SetLast%20Time%20Tower%20Fired (Utilities|Time|GetGameTimeinSeconds))
  (Utilities|FlowControl|Sequence
    (:then_0
      (goto _label Reset))
    (:then_1
      (Utilities|FlowControl|DoN (Variables|Default|GetFireHowManyAtOnce) :!label _label
        (:Exit
          (Utilities|IsValid (Variables|Default|GetTarget)
            (:Is%20Valid
              (CallFunction|SwordSwing)
              (goto _label))))))))