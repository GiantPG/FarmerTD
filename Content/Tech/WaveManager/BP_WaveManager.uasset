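; Wave manager that creates the wave UI and spawns enemies in timed subwaves after a countdown.
; A looping timer updates the UI, then subwaves chain recursively through data table rows, mapping seed types to classes and passing each enemy its spawn point's spline.
; A missing row resets the subwave index and restarts the countdown.
; Death checks can advance the wave, but live spawning never fills the enemy list; older spawn logic is disconnected.
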(event Custom|Start%20Countdown
  ;[1 1 1] Countdown
  (bind _returnvalue (Utilities|Time|SetTimerbyEvent (delegate Custom|Count) 1.0 true))
  (Variables|Default|SetCountdown (Variables|Default|GetCountdownDuration)))

(event Custom|Count
  (bind _countdown (Variables|Default|GetCountdown))
  ;[1 1 1] Countdown
  (bind _aswb_wave_ui (Utilities|Casting|CastToWB_WaveUI (Variables|Default|GetWaveUIRef)))
  (Default|SetTimer _aswb_wave_ui _countdown)
  (if (== _countdown 0)
    (Utilities|Time|ClearandInvalidateTimerbyHandle (stale Custom|Start%20Countdown _returnvalue))
    (CallFunction|StartWave)
    (else
      (Math|Integer|DecrementInt (Variables|Default|GetCountdown)))))

(event Custom|Start%20Wave
  ;[1 1 1] Start wave
  (CallFunction|SpawnSubwave))

(event Custom|Start%20Check%20If%20Enemies%20Are%20Dead
  ;[1 1 1] Check if enemies are dead, and start new wave
  (bind _aredead_1 (CallFunction|CheckifAllEnemiesDead :!label _label))
  (if _aredead_1
    (Math|Integer|IncrementInt (Variables|Default|GetWaveNumber)
      (:%20%20
        (CallFunction|StartCountdown)))
    (else
      (Utilities|FlowControl|Delay 1.0)
      (goto _label))))

(event Custom|EnemyDeath
  (params (Enemy :type BP%20Base%20Enemy%20Object%20Reference))
  (bind _currentenemies (Variables|Default|GetCurrentEnemies))
  ;[1 1 1] Enemy Death
  (Utilities|Array|RemoveItem _currentenemies Enemy)
  (if (and (== (Utilities|Array|Length _currentenemies) 0) (Variables|Default|GetFinishedSpawning))
    (Math|Integer|IncrementInt (Variables|Default|GetWaveNumber)
      (:%20%20
        (CallFunction|StartCountdown)))))

(event Custom|Spawn%20Subwave
  ;[1 1 1] Spawn Subwave
  (bind _returnvalue (Utilities|GetDataTableRow (Variables|Default|GetEnemyDataTable) (Utilities|String|StringToName (Utilities|String|ToString(Integer) (Variables|Default|GetSubWaveNumber))))
    (:then
      (Utilities|ForLoopwithDelay 1 (.NumberOfEnemies (Utilities|Struct|BreakSubWaveInfo _returnvalue)) (.Delay (Utilities|Struct|BreakSubWaveInfo _returnvalue))
        (:Loop%20Body
          (bind _returnvalue_2 (Game|SpawnActorfromClass (.Value (Utilities|Map|Find (Variables|Default|GetSeedToClass) (.SeedType (Utilities|Struct|BreakSubWaveInfo _returnvalue)))) (Transformation|GetActorTransform (Utilities|Array|Get(acopy) (Variables|Default|GetEnemySpawnPoints) (.SpawnPointNumber (Utilities|Struct|BreakSubWaveInfo _returnvalue)))) "Undefined" 0 0))
          (Class|BPIInitable|Init(Message) _returnvalue_2 (.SeedType (Utilities|Struct|BreakSubWaveInfo _returnvalue)) (Variables|/Game/Tech/WaveManager/BP_EnemySpawner.BP_EnemySpawner_C|GetSpline (Utilities|Array|Get(acopy) (Variables|Default|GetEnemySpawnPoints) (.SpawnPointNumber (Utilities|Struct|BreakSubWaveInfo _returnvalue)))) self))
        (:Completed
          (Math|Integer|IncrementInt (Variables|Default|GetSubWaveNumber)
            (:%20%20
              (Utilities|FlowControl|Delay (.TimeUntilNextSubwave (Utilities|Struct|BreakSubWaveInfo _returnvalue)))
              (CallFunction|SpawnSubwave))))))
    (:RowNotFound
      (Variables|Default|SetSubWaveNumber 1)
      (CallFunction|StartCountdown))))

(event Custom|PreWavePhase)

(event EventBeginPlay
  ;[1 1 1] Begin Countdown + Create UI
  (CallFunction|StartCountdown)
  (bind _returnvalue (UserInterface|CreateWidget "/Game/Tech/WaveManager/WB_WaveUI.WB_WaveUI_C"))
  (bind _output_get (Variables|Default|SetWaveUIRef _returnvalue))
  (UserInterface|Viewport|AddtoViewport _output_get 0)
  (bind _aswb_wave_ui (Utilities|Casting|CastToWB_WaveUI (Variables|Default|GetWaveUIRef)))
  (Default|SetWave _aswb_wave_ui (Variables|Default|GetWaveNumber) 1))

(fn ConstructionScript)

(fn SpawnEnemies
  (params (EnemyInfo :type Enemy%20Info%20Structure%20%28by%20ref%29)))

(fn CheckifAllEnemiesDead
  (LocalVariables|SetAreDead? true)
  (for _array_element (Variables|Default|GetCurrentEnemies)
    (Utilities|IsValid _array_element
      (:Is%20Valid
        (LocalVariables|SetAreDead? false))))
  (return (LocalVariables|GetAreDead?)))