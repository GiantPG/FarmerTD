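; BP_EnemySpawner is a spawner actor that creates waves of BP_EnemyTest enemies at its own transform.
; On BeginPlay it binds StartWave to the SpawnNextWave dispatcher on BP_ThirdPersonGameMode.
; Each wave waits for a countdown, then spawns the whole batch at once, adjusting for collisions but always spawning.
; The batch size then grows by an increment that itself rises by one per wave.
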(event Custom|StartWave
  (Utilities|FlowControl|Delay (Math|Conversions|ToFloat(Integer) (Variables|Default|GetCountdown)))
  (for _index (range 0 (- (Variables|Default|GetEnemySpawned) 1))
    (Game|SpawnActorfromClass "/Game/Tech/WaveManager/BP_EnemyTest.BP_EnemyTest_C" (Transformation|GetActorTransform) "AdjustIfPossibleButAlwaysSpawn" 0 0))
  ;[1 1 1] Every time enemies are spawned the amount spawned next is increased exponentially (not sure if we need it, can delete if not)
  (Math|Integer|IncrementInt (Variables|Default|GetEnemyIncrement)
    (:%20%20
      (Variables|Default|SetEnemySpawned (+ (Variables|Default|GetEnemySpawned) (Variables|Default|GetEnemyIncrement))))))

(event EventBeginPlay
  (bind _asbp_third_person_game_mode (Utilities|Casting|CastToBP_ThirdPersonGameMode (Game|GetGameMode)))
  (EventDispatchers|AssignSpawnNextWave _asbp_third_person_game_mode (delegate Custom|StartWave)))

(fn ConstructionScript)