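; Chilli projectile that spawns a BP_ChilliFire actor at its Arrow component's location when its collision sphere hits something, then destroys itself.
; If nothing is hit, it destroys itself after a short delay from BeginPlay.
; BeginPlay also gathers BP_PotatoTower actors, but only an unconnected sphere-trace area-damage chain uses them, reading the first tower's SDamage.
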(event OnComponentHit(SphereCollision)
  (params (HitComponent :type Primitive%20Component%20Object%20Reference) (OtherActor :type Actor%20Object%20Reference) (OtherComp :type Primitive%20Component%20Object%20Reference) (NormalImpulse :type Vector :default "0, 0, 0") (Hit :type Hit%20Result%20Structure%20%28by%20ref%29))
  (Game|SpawnActorfromClass "/Game/Tech/BaseProjectile/BP_ChilliFire.BP_ChilliFire_C" (Math|Conversions|ToTransform(Vector) (Transformation|GetWorldLocation (Variables|Default|GetArrow))) "Undefined" 0 0)
  (Actor|DestroyActor))

(event OnComponentBeginOverlap(SphereCollision)
  (params (OverlappedComponent :type Primitive%20Component%20Object%20Reference) (OtherActor :type Actor%20Object%20Reference) (OtherComp :type Primitive%20Component%20Object%20Reference) (OtherBodyIndex :type Integer) (bFromSweep :type Boolean) (SweepResult :type Hit%20Result%20Structure%20%28by%20ref%29)))

(event EventBeginPlay
  (bind _outactors (Actor|GetAllActorsOfClass "/Game/Tech/BaseTower/BP_PotatoTower.BP_PotatoTower_C"))
  (Utilities|FlowControl|Delay 5.0)
  (Actor|DestroyActor))

(fn ConstructionScript)