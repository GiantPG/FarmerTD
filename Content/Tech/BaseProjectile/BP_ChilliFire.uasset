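; BP_ChilliFire is a fire area actor for the Chilli tower that deals damage and destroys itself after three seconds.
; BeginPlay copies damage from the first Chilli tower found and scales its flattened mesh to that tower's range.
; Tick calls FireAOE, damaging one cached BP_BaseEnemy every frame, regardless of overlap.
; Mesh overlap only sets a zero-time timer, so it does not select targets.
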(event OnComponentBeginOverlap(StaticMesh)
  (params (OverlappedComponent :type Primitive%20Component%20Object%20Reference) (OtherActor :type Actor%20Object%20Reference) (OtherComp :type Primitive%20Component%20Object%20Reference) (OtherBodyIndex :type Integer) (bFromSweep :type Boolean) (SweepResult :type Hit%20Result%20Structure%20%28by%20ref%29))
  (Utilities|Time|SetTimerbyEvent (EventDispatchers|CreateEvent :!event Custom|FireAOE) 0.0))

(event Custom|FireAOE
  (Game|Damage|ApplyDamage (Variables|Default|GetAs%20BP%20Base%20Enemy) (Variables|Default|GetDamageFireOuchies) 0 0)
  (Utilities|FlowControl|Delay 3.0)
  (Actor|DestroyActor))

(event EventBeginPlay
  (bind _returnvalue (Actor|GetActorOfClass "/Game/Tech/BaseTower/BP_TowerBaseTestNewDetectionChilli.BP_TowerBaseTestNewDetectionChilli_C"))
  (bind _output_get (Variables|Default|SetChilliTowerRef _returnvalue))
  (Variables|Default|SetDamageFireOuchies (Variables|/Game/Tech/BaseTower/BP_TowerBaseTestNewDetection.BP_TowerBaseTestNewDetection_C|GetS%20Damage _output_get))
  (bind _returnvalue_2 (Actor|GetActorOfClass "/Game/Tech/Enemies/BP_BaseEnemy.BP_BaseEnemy_C"))
  (Variables|Default|SetAs%20BP%20Base%20Enemy _returnvalue_2)
  (Transformation|SetWorldScale3D (Variables|Default|GetStaticMesh) (Math|Vector|MakeVector (/ (Variables|/Game/Tech/BaseTower/BP_TowerBaseTestNewDetection.BP_TowerBaseTestNewDetection_C|GetS%20Tower%20Range (Variables|Default|GetChilliTowerRef)) 1.3e+02) (/ (Variables|/Game/Tech/BaseTower/BP_TowerBaseTestNewDetection.BP_TowerBaseTestNewDetection_C|GetS%20Tower%20Range (Variables|Default|GetChilliTowerRef)) 1.3e+02) 0.0)))

(event Collision|EventActorBeginOverlap
  (params (OtherActor :type Actor%20Object%20Reference)))

(event EventTick
  (params (DeltaSeconds :type Float%20%28single-precision%29))
  (CallFunction|FireAOE))

(fn ConstructionScript)