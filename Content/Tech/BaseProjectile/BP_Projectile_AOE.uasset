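; BP_Projectile_AOE is a tower projectile that deals area damage when its collision sphere begins an overlap.
; The overlap runs a multi-sphere trace at the mesh location on the Visibility channel, with persistent debug drawing.
; Its loop damages hit actors using SDamage from the first tower found at BeginPlay, calling DestroyActor inside the loop.
; Otherwise, the projectile destroys itself after a short delay.
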(event OnComponentBeginOverlap(SphereCollision)
  (params (OverlappedComponent :type Primitive%20Component%20Object%20Reference) (OtherActor :type Actor%20Object%20Reference) (OtherComp :type Primitive%20Component%20Object%20Reference) (OtherBodyIndex :type Integer) (bFromSweep :type Boolean) (SweepResult :type Hit%20Result%20Structure%20%28by%20ref%29))
  (bind _staticmesh (Variables|Default|GetStaticMesh))
  (bind _returnvalue (Transformation|GetWorldLocation _staticmesh))
  (bind _outhits (Collision|MultiSphereTraceByChannel _returnvalue _returnvalue (Variables|Default|GetRadius) "TraceTypeQuery1" false 0 "Persistent"))
  (for _array_element _outhits
    (Development|PrintString "Projectile Hit" false)
    (Development|PrintString (Utilities|GetDisplayName (.hitactor _array_element)))
    (Game|Damage|ApplyDamage (.hitactor _array_element) (Variables|/Game/Tech/BaseTower/BP_TowerBaseTestNewDetection.BP_TowerBaseTestNewDetection_C|GetS%20Damage (Utilities|Array|Get(acopy) (stale EventBeginPlay _outactors))) 0 0)
    (Actor|DestroyActor)))

(event EventBeginPlay
  (bind _outactors (Actor|GetAllActorsOfClass "/Game/Tech/BaseTower/BPC_TowerBaseTestNewDetectionPotato.BPC_TowerBaseTestNewDetectionPotato_C"))
  (Utilities|FlowControl|Delay 5.0)
  (Actor|DestroyActor))

(fn ConstructionScript)