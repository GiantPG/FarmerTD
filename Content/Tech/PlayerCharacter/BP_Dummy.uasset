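; BP_Dummy is a player character Blueprint with a watering can action and a follow camera whose relative location is cached at construction.
; Water runs a stationary multi-sphere trace just ahead of the actor and sends TransferWaterMessage to each WorldDynamic hit.
; Each use with water remaining drains the can by its efficiency, clamped to capacity, then calls AdjustSpeed, even without a hit.
; UpdateUI is an empty stub.
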(fn ConstructionScript
  (Variables|Default|SetCameraLocation (Variables|/Script/Engine.SceneComponent|GetRelativeLocation (Variables|Camera|GetFollowCamera))))

(fn Water
  (bind _returnvalue (Transformation|GetActorLocation))
  (bind _returnvalue_2 (Transformation|GetActorForwardVector))
  (bind _returnvalue_3 (* _returnvalue_2 1e+02))
  (bind _returnvalue_4 (+ _returnvalue _returnvalue_3))
  (if (> (Variables|Character|GetWaterLevel) 0.0)
    (bind (_outhits _returnvalue_5) (Collision|MultiSphereTraceForObjects _returnvalue_4 _returnvalue_4 25.0 (Utilities|Array|MakeArray "ObjectTypeQuery2") false 0 "None"))
    (if _returnvalue_5
      (for _array_element _outhits
        (Class|BPIWaterTransferable|TransferWater(Message) (.hitactor _array_element) (Variables|Character|GetWateringCanEfficiency))))
    (Variables|Character|SetWaterLevel (Math|Float|Clamp(Float) (- (Variables|Character|GetWaterLevel) (Variables|Character|GetWateringCanEfficiency)) 0.0 (Variables|Character|GetWateringCanCapacity)))
    (CallFunction|AdjustSpeed)))

(fn UpdateUI
  (params (NumberSlot :type Text%20Block%20Object%20Reference) (NewAmount :type Integer)))