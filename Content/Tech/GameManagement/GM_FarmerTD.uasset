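; GM_FarmerTD is the game mode Blueprint for FarmerTD, keeping a list of connected player controllers.
; PostLogin and OnLogout add and remove each BP_PlayerController in the Controllers array, ignoring other controller types.
; An unconnected loop that would spawn a BP_FarmerTed_SpriteMinimap pawn for each controller and possess it never runs.
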(event EventBeginPlay)

(event EventTick
  (params (DeltaSeconds :type Float%20%28single-precision%29)))

(event EventPostLogin
  (params (NewPlayer :type Player%20Controller%20Object%20Reference))
  ;[1 1 1] Controller Login/out
  (bind _asbp_player_controller (Utilities|Casting|CastToBP_PlayerController NewPlayer))
  (Utilities|Array|Add (Variables|Default|GetControllers) _asbp_player_controller))

(event EventOnLogout
  (params (ExitingController :type Controller%20Object%20Reference))
  ;[1 1 1] Controller Login/out
  (bind _asbp_player_controller (Utilities|Casting|CastToBP_PlayerController ExitingController))
  (Utilities|Array|RemoveItem (Variables|Default|GetControllers) _asbp_player_controller))

(fn ConstructionScript)