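; Sweetcorn cob enemy, a child class that names itself "Sweetcorn" on BeginPlay and spawns a sweetcorn kernel enemy.
; Its SpawnKernels override calls the parent, then traces 200 units down from the cob and spawns one BP_SweetcornKernelEnemy at the hit location.
; The trace ignores the player character so the kernel does not spawn on the player.
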(event Custom|Init_2
  (params (SeedType :type ENUM_SeedTypes%20Enum :default "NewEnumerator0") (SplineToFollow :type Spline%20Component%20Object%20Reference) (WaveManager :type BP%20Wave%20Manager%20Object%20Reference)))

(event EventBeginPlay
  (Variables|Default|SetName "Sweetcorn")
  (|CallParentFunction))

(fn ConstructionScript
  (|CallParentFunction))

(fn SpawnKernels
  (bind _returnvalue (Transformation|GetActorLocation))
  ;[1 1 1] Spawns SweetcornKernel
  (|CallParentFunction)
  (bind _outhit (Collision|LineTraceByChannel _returnvalue (- _returnvalue "0.000000,0.000000,200.000000") "TraceTypeQuery1" false (Utilities|Array|MakeArray (Game|GetPlayerCharacter 0)) "None")) ; Shoots linetrace down to get spawn location
  (Game|SpawnActorfromClass "/Game/Tech/EnemyClasses/EnemyClasses/BP_SweetcornKernelEnemy.BP_SweetcornKernelEnemy_C" (Math|Transform|MakeTransform (.Location (Collision|BreakHitResult _outhit))) "Undefined" 0 0) ; Gets correct actor to spawn
)