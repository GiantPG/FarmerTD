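; BP_CarrotEnemy is the carrot enemy, a child Blueprint that passes BeginPlay and Init, which takes a spline to follow and a wave manager, to its parent.
; Its construction script runs the parent's, then looks up its class enum name in the enemy stats DataTable.
; When the row is found, it sets current health, speed and damage from that row, keeping these stats data-driven.
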(event EventInit
  (params (SplineToFollow :type Spline%20Component%20Object%20Reference) (WaveManager :type BP%20Wave%20Manager%20Object%20Reference))
  (|CallParentFunction SplineToFollow WaveManager))

(event EventBeginPlay
  (|CallParentFunction))

(fn ConstructionScript
  (|CallParentFunction)
  (bind _returnvalue (Utilities|GetDataTableRow "/Game/Tech/EnemyClasses/EnemyClassStats_DataTable.EnemyClassStats_DataTable" (Utilities|Name|EnumtoName (Variables|Default|GetENUM_Class)))
    (:then
      (Variables|Default|SetCurrentHealth (.Health (Utilities|Struct|BreakS_EnemyClassStats _returnvalue)))
      (Variables|Default|SetSpeed (.Speed (Utilities|Struct|BreakS_EnemyClassStats _returnvalue)))
      (Variables|Default|SetDamage (.Damage (Utilities|Struct|BreakS_EnemyClassStats _returnvalue))))))