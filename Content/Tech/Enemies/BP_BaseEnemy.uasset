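; Base enemy actor for a wave-based mode that travels along a spline and can be killed.
; Init takes the spline, wave manager and seed type, loading health, speed and damage from a data table row named after the type.
; A timeline, rate-scaled by speed over spline length, drives X/Y position and tangent-facing rotation while keeping Z.
; AnyDamage reduces health, notifying the wave manager and destroying the actor at zero.
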(event Custom|MoveAlongSpline
  (bind _splinetofollow (Variables|Default|GetSplineToFollow))
  (bind _splinetofollow_2 (Variables|Default|GetSplineToFollow))
  ;[1 1 1 1 36] Movement
  (bind _alpha (Timeline|Timeline_Move PlayFromStart)
    (:Update
      (Utilities|IsValid _splinetofollow_2
        (:Is%20Valid
          (Transformation|SetActorLocationAndRotation (Math|Vector|MakeVector (.x (Spline|GetLocationatDistanceAlongSpline _splinetofollow_2 (Math|Float|Lerp 0.0 (Spline|GetDistanceAlongSplineatSplinePoint _splinetofollow (- (Spline|GetNumberOfSplinePoints _splinetofollow) 1)) _alpha) "World")) (.y (Spline|GetLocationatDistanceAlongSpline _splinetofollow_2 (Math|Float|Lerp 0.0 (Spline|GetDistanceAlongSplineatSplinePoint _splinetofollow (- (Spline|GetNumberOfSplinePoints _splinetofollow) 1)) _alpha) "World")) (.z (Transformation|GetActorLocation))) (Math|Conversions|RotationFromXVector (Spline|GetTangentatDistanceAlongSpline (Variables|Default|GetSplineToFollow) (Math|Float|Lerp 0.0 (Spline|GetDistanceAlongSplineatSplinePoint _splinetofollow (- (Spline|GetNumberOfSplinePoints _splinetofollow) 1)) _alpha) "World"))))))))

(event EventInit
  (params (SplineToFollow :type Spline%20Component%20Object%20Reference) (WaveManager :type BP%20Wave%20Manager%20Object%20Reference) (SeedType :type ENUM_SeedTypes%20Enum :default "NewEnumerator0"))
  ;[1 1 1 1 36] Init
  (bind _returnvalue (Utilities|GetDataTableRow "/Game/Tech/EnemyClasses/EnemyClassStats_DataTable.EnemyClassStats_DataTable" (Utilities|String|StringToName (Utilities|String|EnumtoString SeedType)))
    (:then
      (Variables|Default|SetCurrentHealth (.Health (Utilities|Struct|BreakS_EnemyClassStats _returnvalue)))
      (Variables|Default|SetSpeed (.Speed (Utilities|Struct|BreakS_EnemyClassStats _returnvalue)))
      (Variables|Default|SetDamage (.Damage (Utilities|Struct|BreakS_EnemyClassStats _returnvalue)))
      (bind _output_get (Variables|Default|SetSplineToFollow SplineToFollow))
      (Variables|Default|SetWaveManager WaveManager)
      (Components|Timeline|SetPlayRate (Variables|Default|GetTimeline_Move) (/ 1.0 (/ (Spline|GetSplineLength _output_get) (Variables|Default|GetSpeed))))
      (CallFunction|MoveAlongSpline))))

(event EventBeginPlay)

(event Game|Damage|EventAnyDamage
  (params (Damage :type Float%20%28single-precision%29) (DamageType :type Damage%20Type%20Object%20Reference) (InstigatedBy :type Controller%20Object%20Reference) (DamageCauser :type Actor%20Object%20Reference))
  ;[1 1 1 1 36] Damage
  (bind _output_get (Variables|Default|SetCurrentHealth (- (Variables|Default|GetCurrentHealth) Damage)))
  (if (<= _output_get 0.0)
    (Default|EnemyDeath (Variables|Default|GetWaveManager) self)
    (Actor|DestroyActor)))

(fn ConstructionScript)