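; Base enemy for a wave-based tower defense game that follows a spline path and drops a coin on death.
; EnemyInit loads stats from a data table by seed type, then a timeline drives movement and rotation along the spline.
; Damage, reduced by resistance, updates the health widget or notifies the wave manager and destroys the enemy.
; Events handle slow and resistance buffs, though SetSpeed is an empty stub here.
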(event Custom|MoveAlongSpline
  (bind _splinetofollow (Variables|Default|GetSplineToFollow))
  (bind _splinetofollow_2 (Variables|Default|GetSplineToFollow))
  ;[1 1 1 1 36] Movement
  (bind _alpha (Timeline|Timeline_0 PlayFromStart)
    (:Update
      (Utilities|IsValid _splinetofollow_2
        (:Is%20Valid
          (Transformation|SetActorLocationAndRotation (Math|Vector|MakeVector (.x (Spline|GetLocationatDistanceAlongSpline _splinetofollow_2 (Math|Float|Lerp 0.0 (Spline|GetDistanceAlongSplineatSplinePoint _splinetofollow (- (Spline|GetNumberOfSplinePoints _splinetofollow) 1)) _alpha) "World")) (.y (Spline|GetLocationatDistanceAlongSpline _splinetofollow_2 (Math|Float|Lerp 0.0 (Spline|GetDistanceAlongSplineatSplinePoint _splinetofollow (- (Spline|GetNumberOfSplinePoints _splinetofollow) 1)) _alpha) "World")) (.z (Transformation|GetActorLocation))) (Math|Conversions|RotationFromXVector (Spline|GetTangentatDistanceAlongSpline (Variables|Default|GetSplineToFollow) (Math|Float|Lerp 0.0 (Spline|GetDistanceAlongSplineatSplinePoint _splinetofollow (- (Spline|GetNumberOfSplinePoints _splinetofollow) 1)) _alpha) "World"))))))))

(event Custom|Init%20HUD
  ;[1 1 1] Init HUD
  (bind _asenemy_ui (Utilities|Casting|CastToenemyUI (UserInterface|GetWidget (Variables|Default|GetWidget))))
  (Default|SetName _asenemy_ui (Variables|Default|GetName)))

(event Custom|CustomEvent_2
  ;[1 1 1] Restore Speed
  (Variables|Default|SetEnemyStats (Utilities|Struct|MakeS_EnemyClassStats (.health (Variables|Default|GetEnemyStats)) (.maxspeed (Variables|Default|GetEnemyStats)) (.damage (Variables|Default|GetEnemyStats)) (.maxhealth (Variables|Default|GetEnemyStats)) (.maxspeed (Variables|Default|GetEnemyStats)) (.damageresistance (Variables|Default|GetEnemyStats)))))

(event Custom|CustomEvent_3
  (params (BuffAmount :type Float%20%28double-precision%29))
  ;[1 1 1] Buff
  (Variables|Default|SetEnemyStats (Utilities|Struct|MakeS_EnemyClassStats (.health (Variables|Default|GetEnemyStats)) (.speed (Variables|Default|GetEnemyStats)) (.damage (Variables|Default|GetEnemyStats)) (.maxhealth (Variables|Default|GetEnemyStats)) (.maxspeed (Variables|Default|GetEnemyStats)) BuffAmount)))

(event Custom|CustomEvent_4
  ;[1 1 1] Debuff
  (Variables|Default|SetEnemyStats (Utilities|Struct|MakeS_EnemyClassStats (.health (Variables|Default|GetEnemyStats)) (.speed (Variables|Default|GetEnemyStats)) (.damage (Variables|Default|GetEnemyStats)) (.maxhealth (Variables|Default|GetEnemyStats)) (.maxspeed (Variables|Default|GetEnemyStats)) 0.0)))

(event Custom|CustomEvent
  (params (Amount :type Float%20%28double-precision%29))
  ;[1 1 1] Slow
  (CallFunction|SetSpeed (Variables|Default|GetSplineToFollow) (* (.maxspeed (Variables|Default|GetEnemyStats)) Amount)))

(event Custom|CustomEvent_1
  (params (Tower :type BP%20Tower%20Base%20Object%20Reference)))

(event EventBeginPlay
  (CallFunction|InitHUD))

(event Game|Damage|EventAnyDamage
  (params (Damage :type Float%20%28single-precision%29) (DamageType :type Damage%20Type%20Object%20Reference) (InstigatedBy :type Controller%20Object%20Reference) (DamageCauser :type Actor%20Object%20Reference))
  (bind _returnvalue (Transformation|GetActorTransform))
  ;[1 1 1 1 36] Damage
  ;;[1 1 1] Set new current health after damage
  (bind _output_get (Variables|Default|SetEnemyStats (Utilities|Struct|MakeS_EnemyClassStats (- (.health (Variables|Default|GetEnemyStats)) (- Damage (.damageresistance (Variables|Default|GetEnemyStats)))) (.speed (Variables|Default|GetEnemyStats)) (.damage (Variables|Default|GetEnemyStats)) (.maxhealth (Variables|Default|GetEnemyStats)) (.maxspeed (Variables|Default|GetEnemyStats)) (.damageresistance (Variables|Default|GetEnemyStats)))))
  ;;[1 1 1] Check if health below or equal to 0
  (if (<= (.health _output_get) 0.0)
    ;;[1 1 1] If dead notify wave manager, drop coin and destroy self
    (Default|EnemyDeath (Variables|Default|GetWaveManager))
    (Game|SpawnActorfromClass "/Game/Tech/Collectables/BP_Coin.BP_Coin_C" (Math|Transform|MakeTransform (Math|Vector|MakeVector (.x (.location _returnvalue)) (.y (.location _returnvalue)) 0.0) "0, 0, 0" "1.000000,1.000000,1.000000") "Undefined" 0 (Variables|Default|GetCoinValue) 0)
    (Actor|DestroyActor)
    (else
      ;;[1 1 1] If still alive update UI
      (Default|SetHealth (Variables|Default|GetEnemy%20UI) (/ (.health (Variables|Default|GetEnemyStats)) (.maxhealth (Variables|Default|GetEnemyStats)))))))

(event EventEnemyInit
  (params (SeedType :type ENUM_SeedTypes%20Enum :default "NewEnumerator0") (SplineToFollow :type Spline%20Component%20Object%20Reference) (WaveManager :type BP%20Wave%20Manager%20Object%20Reference))
  ;[1 1 1 1 36] Init
  (bind _returnvalue (Utilities|GetDataTableRow "/Game/Tech/EnemyClasses/EnemyClassStats_DataTable.EnemyClassStats_DataTable" (Utilities|String|StringToName (Utilities|String|EnumtoString SeedType)))
    (:then
      (Variables|Default|SetEnemyStats _returnvalue)
      (bind _output_get (Variables|Default|SetSplineToFollow SplineToFollow))
      (CallFunction|SetSpeed _output_get (.maxspeed (Variables|Default|GetEnemyStats)))
      (Variables|Default|SetWaveManager WaveManager)
      (CallFunction|MoveAlongSpline)
      (bind _asenemy_ui (Utilities|Casting|CastToenemyUI (UserInterface|GetWidget (Variables|Default|GetWidget))))
      (Variables|Default|SetEnemy%20UI _asenemy_ui))))

(fn ConstructionScript)

(fn SetSpeed
  (params (SplinetoFollow :type Spline%20Component%20Object%20Reference) (Speed :type Float%20%28double-precision%29)))