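; BP_Shop is a world shop that lets the Farmer Ted player open and close a shop menu while standing nearby.
; Box overlap shows or hides a prompt widget, toggles the actor's input and opens or closes a gate on Interact.
; Interact lazily creates WB_ShopUI, then uses the paused state to toggle the menu, pause, mouse cursor, input mode and Ted's HUD visibility.
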(event OnComponentBeginOverlap(Box)
  (params (OverlappedComponent :type Primitive%20Component%20Object%20Reference) (OtherActor :type Actor%20Object%20Reference) (OtherComp :type Primitive%20Component%20Object%20Reference) (OtherBodyIndex :type Integer) (bFromSweep :type Boolean) (SweepResult :type Hit%20Result%20Structure%20%28by%20ref%29))
  (bind _returnvalue (Game|GetPlayerController 0))
  (bind _tedref (Variables|Default|GetTedRef))
  (bind _hud_ref (Variables|/Game/Tech/PlayerCharacter/BP_FarmerTed_SpriteMinimap.BP_FarmerTed_SpriteMinimap_C|GetHUD%20Ref _tedref))
  (Utilities|Casting|CastToBP_FarmerTed_SpriteMinimap OtherActor)
  (Input|EnableInput (Game|GetPlayerController 0))
  (Development|SetHiddeninGame (Variables|Default|GetWidget) false false)
  (Variables|Default|SetPlayerNearShop true)
  (Utilities|FlowControl|Gate true) ; enters at Open
)

(event OnComponentEndOverlap(Box)
  (params (OverlappedComponent :type Primitive%20Component%20Object%20Reference) (OtherActor :type Actor%20Object%20Reference) (OtherComp :type Primitive%20Component%20Object%20Reference) (OtherBodyIndex :type Integer))
  (bind _returnvalue (Game|GetPlayerController 0))
  (bind _tedref (Variables|Default|GetTedRef))
  (bind _hud_ref (Variables|/Game/Tech/PlayerCharacter/BP_FarmerTed_SpriteMinimap.BP_FarmerTed_SpriteMinimap_C|GetHUD%20Ref _tedref))
  (Utilities|Casting|CastToBP_FarmerTed_SpriteMinimap OtherActor)
  (Input|DisableInput (Game|GetPlayerController 0))
  (Development|SetHiddeninGame (Variables|Default|GetWidget) true false)
  (Variables|Default|SetPlayerNearShop false)
  (Utilities|FlowControl|Gate true) ; enters at Close
)

(event EventBeginPlay
  (bind _returnvalue (Actor|GetActorOfClass "/Game/Tech/PlayerCharacter/BP_FarmerTed_SpriteMinimap.BP_FarmerTed_SpriteMinimap_C"))
  (Variables|Default|SetTedRef _returnvalue))

(event Input|ActionEvents|InputActionInteract
  (params (Key :type Key%20Structure :default "None"))
  (bind _returnvalue (Game|GetPlayerController 0))
  (bind _tedref (Variables|Default|GetTedRef))
  (bind _hud_ref (Variables|/Game/Tech/PlayerCharacter/BP_FarmerTed_SpriteMinimap.BP_FarmerTed_SpriteMinimap_C|GetHUD%20Ref _tedref))
  (:Pressed
    (Utilities|FlowControl|Gate true
      (:Exit
        (if (Variables|Default|GetPlayerNearShop)
          (Utilities|IsValid (Variables|Default|GetShopUIRef)
            (:Is%20Valid
              _)
            (:Is%20Not%20Valid
              (bind _returnvalue_2 (UserInterface|CreateWidget "/Game/Tech/Shop/ShopWidgets/WB_ShopUI.WB_ShopUI_C" 0 self))
              (Variables|Default|SetShopUIRef _returnvalue_2)))
          (if (Game|IsGamePaused)
            (Widget|RemovefromParent (Variables|Default|GetShopUIRef))
            (Game|SetGamePaused false)
            (Variables|/Script/Engine.PlayerController|SetbShowMouseCursor _returnvalue false)
            (Input|SetInputModeGameOnly _returnvalue false)
            (Variables|/Script/UMG.Widget|SetVisibility _hud_ref "Visible")
            (else
              (UserInterface|Viewport|AddtoViewport (Variables|Default|GetShopUIRef) 0)
              (Game|SetGamePaused true)
              (Variables|/Script/Engine.PlayerController|SetbShowMouseCursor _returnvalue true)
              (Input|SetInputModeGameandUI _returnvalue (Variables|Default|GetShopUIRef) "LockInFullscreen" false false)
              (Variables|/Script/UMG.Widget|SetVisibility _hud_ref "Hidden"))))))))

(fn ConstructionScript)